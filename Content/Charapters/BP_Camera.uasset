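; Player camera that doubles as the game's hub for UI, audio and the three-tier coin economy.
; A looping timer drives WASD and wheel movement through gates, with opposing counters limiting travel.
; It creates and swaps menu and HUD widgets, passing the HUD to machines and platforms.
; Runtime-created audio components provide music and event sounds with random meme variants; ChangeCoins handles payments, and a timer clamps negative bronze.
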(event Custom|Nen0Dengi
  ;[0.15 0.15 0.15 0.5] Anti-CoinsValue
  (if (< (Variables|Default|GetBronze_Coin) 0)
    (Variables|Default|SetBronze_Coin 0)))

(event Custom|MovementTimer
  ;[0.15 0.15 0.15 0.5] Movement
  (Utilities|Time|SetTimerbyEvent (delegate Custom|Move) 0.005 true))

(event Custom|SettingsUI
  ;[0.15 0.15 0.15 0.5] UI
  ;;[0.15 0.15 0.15 0.5] Settings
  (Viewport|RemoveAllWidgets)
  (UserInterface|Viewport|AddtoViewport (Variables|Default|GetWBP_Settings) 0))

(event Custom|MenuUI
  ;[0.15 0.15 0.15 0.5] UI
  ;;[0.15 0.15 0.15 0.5] Menu
  (Viewport|RemoveAllWidgets)
  (UserInterface|Viewport|AddtoViewport (Variables|Default|GetWBP_Menu) 0))

(event Custom|ResetSettingsMusic
  ;[0.15 0.15 0.15 0.5] UI
  ;;[0.15 0.15 0.15 0.5] MainMenu
  (Utilities|FlowControl|DoOnce false) ; enters at Reset
)

(event Custom|MusicValue
  (params (Value :type Float%20%28double-precision%29))
  ;[0.15 0.15 0.15 0.5] Music/Sound volume
  (Utilities|FlowControl|Delay 0.2)
  (Audio|Components|Audio|SetVolumeMultiplier (Variables|Default|GetSW_InGame) Value :!class /Script/Engine.AudioComponent))

(event Custom|ConstructMusic
  ;[0.15 0.1473 0 0.5] MAIN
  ;;[0.15 0.15 0.15 0.5] AddAudioComponent
  (bind _returnvalue (AddComponent|AddAudioComponent false))
  (Variables|Default|SetSW_InGame _returnvalue)
  (bind _returnvalue_2 (AddComponent|AddAudioComponent false))
  (Variables|Default|SetSW_InMenu _returnvalue_2)
  (bind _returnvalue_3 (AddComponent|AddAudioComponent false))
  (bind _output_get (Variables|Default|SetSW_BGMachinesWorking _returnvalue_3))
  (Audio|Components|Audio|Stop (Variables|Default|GetSW_InGame))
  (bind _returnvalue_4 (AddComponent|AddAudioComponent false))
  (Audio|Components|Audio|Stop _returnvalue_4)
  (Variables|Default|SetSW_Clicking _returnvalue_4)
  (bind _returnvalue_5 (AddComponent|AddAudioComponent false))
  (Audio|Components|Audio|Stop _returnvalue_5)
  (Variables|Default|SetSW_BuyFail _returnvalue_5)
  (bind _returnvalue_6 (AddComponent|AddAudioComponent false))
  (Audio|Components|Audio|Stop _returnvalue_6)
  (Variables|Default|SetSW_Upgrading _returnvalue_6)
  (bind _returnvalue_7 (AddComponent|AddAudioComponent false))
  (Audio|Components|Audio|Stop _returnvalue_7)
  (Variables|Default|SetSW_BuildingNormal _returnvalue_7)
  (bind _returnvalue_8 (AddComponent|AddAudioComponent false))
  (Audio|Components|Audio|Stop _returnvalue_8)
  (Variables|Default|SetSW_BuildingMeme _returnvalue_8)
  (bind _returnvalue_9 (AddComponent|AddAudioComponent false))
  (Audio|Components|Audio|Stop _returnvalue_9)
  (Variables|Default|SetSW_Selling _returnvalue_9)
  (CallFunction|ConstructMusicLine2))

(event Custom|SoundValue
  (params (Value :type Float%20%28double-precision%29))
  ;[0.15 0.15 0.15 0.5] Music/Sound volume
  (Utilities|FlowControl|Delay 0.2)
  (Audio|Components|Audio|SetVolumeMultiplier (Variables|Default|GetSW_Clicking) Value :!class /Script/Engine.AudioComponent))

(event Custom|SoundMachineValue
  (params (Value :type Float%20%28double-precision%29))
  ;[0.15 0.15 0.15 0.5] Music/Sound volume
  (Utilities|FlowControl|Delay 0.2)
  (Variables|Default|SetSoundMachineVolume Value)
  (Default|CallEDSoundMachineVolume))

(event Custom|Effects
  (params (Effects :type Boolean))
  ;[0.15 0.15 0.15 0.5] Effects
  (Variables|Default|SetEffect (not Effects))
  (Default|CallEDEffects))

(event Custom|TutorialMenu
  ;[0.15 0.15 0.15 0.5] UI
  ;;[0.15 0.15 0.15 0.5] Menu
  (UserInterface|Viewport|AddtoViewport (Variables|Default|GetWBP_Tutorial) 0))

(event Custom|FalseUpdateSkip
  ;[0.15 0.15 0.15 0.5] FalseUpdateSkip
  (EventDispatchers|BindEventtoEDNotinDialog3 (Variables|Default|GetWBP_Tutorial) (delegate Custom|UpdateDialog3)))

(event Custom|Anti-CoinsValue
  ;[0.15 0.15 0.15 0.5] Anti-CoinsValue
  (Utilities|Time|SetTimerbyEvent (delegate Custom|Nen0Dengi) 0.1 true))

(event Custom|UpdateDialog3
  ;[0.15 0.15 0.15 0.5] FalseUpdateSkip
  (Variables|Default|SetNotInDialog3 (Variables|/Game/Project/Blueprints/UI/Widgets/WBP_Tutorial.WBP_Tutorial_C|GetNotInDialog3 (Variables|Default|GetWBP_Tutorial))))

(event Custom|ConstructMusicLine2
  ;[0.15 0.1473 0 0.5] MAIN
  ;;[0.15 0.15 0.15 0.5] AddAudioComponent
  (bind _returnvalue (AddComponent|AddAudioComponent false))
  (Audio|Components|Audio|Stop _returnvalue)
  (Variables|Default|SetSW_QuestAccepted _returnvalue)
  (bind _returnvalue_2 (AddComponent|AddAudioComponent false))
  (Audio|Components|Audio|Stop _returnvalue_2)
  (Variables|Default|SetSW_QuestAcceptedMeme _returnvalue_2)
  (bind _returnvalue_3 (AddComponent|AddAudioComponent false))
  (Audio|Components|Audio|Stop _returnvalue_3)
  (Variables|Default|SetSW_QuestRefuseMeme _returnvalue_3)
  (bind _returnvalue_4 (AddComponent|AddAudioComponent false))
  (Audio|Components|Audio|Stop _returnvalue_4)
  (Variables|Default|SetSW_QuestRefuse _returnvalue_4))

(event Custom|Move
  ;[0.15 0.15 0.15 0.5] Movement
  (Utilities|FlowControl|Sequence
    (:then_0
      (Utilities|FlowControl|Gate true
        (:Exit
          (Variables|Default|SetWayOfMove 0))))
    (:then_1
      (Utilities|FlowControl|Gate true
        (:Exit
          (Variables|Default|SetWayOfMove 1))))
    (:then_2
      (Utilities|FlowControl|Gate true
        (:Exit
          (Variables|Default|SetWayOfMove 2))))
    (:then_3
      (Utilities|FlowControl|Gate true
        (:Exit
          (Variables|Default|SetWayOfMove 3))))
    (:then_4
      (Utilities|FlowControl|Gate true
        (:Exit
          (Variables|Default|SetWayOfMove 4))))
    (:then_5
      (Utilities|FlowControl|Gate true
        (:Exit
          (Variables|Default|SetWayOfMove 5)))))
  (CallFunction|Movement (Variables|Default|GetWayOfMove)))

(event Custom|Music
  (bind _sw_inmenu (Variables|Default|GetSW_InMenu))
  ;[0.15 0.15 0.15 0.5] Music
  (if (Variables|Default|GetInGame)
    (Audio|Components|Audio|Play (Variables|Default|GetSW_InGame) 0.0)
    (Audio|Components|Audio|Play (Variables|Default|GetSW_BGMachinesWorking) 0.0)
    (if (Audio|Components|Audio|IsPlaying _sw_inmenu)
      (Audio|Components|Audio|Stop _sw_inmenu))
    (else
      (Audio|Components|Audio|Play (Variables|Default|GetSW_InMenu) 0.0)
      (if (Audio|Components|Audio|IsPlaying (Variables|Default|GetSW_InGame))
        (Audio|Components|Audio|Stop (Variables|Default|GetSW_BGMachinesWorking))))))

(event Custom|Sounds
  (params (MailRefuse :type Boolean) (MailAccepted :type Boolean) (Selling :type Boolean) (Building :type Boolean) (Upgrading :type Boolean) (PurchaseFailed :type Boolean))
  ;[0.15 0.15 0.15 0.5] Sounds
  (if MailRefuse
    (if (>= (Math|Random|RandomIntegerinRange 0 100) 10)
      (Audio|Components|Audio|Play (Variables|Default|GetSW_QuestRefuse) 0.0)
      (else
        (Audio|Components|Audio|Play (Variables|Default|GetSW_QuestRefuseMeme) 0.0)))
    (elif MailAccepted
      (if (>= (Math|Random|RandomIntegerinRange 0 100) 10)
        (Audio|Components|Audio|Play (Variables|Default|GetSW_QuestAccepted) 0.0)
        (else
          (Audio|Components|Audio|Play (Variables|Default|GetSW_QuestAcceptedMeme) 0.0)))
      (elif Selling
        (Audio|Components|Audio|Play (Variables|Default|GetSW_Selling) 0.0)
        (elif Building
          (if (>= (Math|Random|RandomIntegerinRange 0 100) 10)
            (Audio|Components|Audio|Play (Variables|Default|GetSW_BuildingNormal) 0.0)
            (else
              (Audio|Components|Audio|Play (Variables|Default|GetSW_BuildingMeme) 0.0)))
          (elif Upgrading
            (Audio|Components|Audio|Play (Variables|Default|GetSW_Upgrading) 0.0)
            (elif PurchaseFailed
              (Audio|Components|Audio|Play (Variables|Default|GetSW_BuyFail) 0.0)
              (else
                (Audio|Components|Audio|Play (Variables|Default|GetSW_Clicking) 0.0)))))))))

(event Custom|GetActorsOfClass
  ;[0.15 0.1473 0 0.5] MAIN
  ;;[0.15 0.15 0.15 0.5] GetActorsOfClass
  (Utilities|FlowControl|Delay 0.1)
  (bind _outactors (Actor|GetAllActorsOfClass "/Game/Project/Blueprints/Actors/Machines/BP_ForMachine.BP_ForMachine_C"))
  (bind _output_get (Variables|Default|SetBP_ForMachine _outactors))
  (for _array_element _output_get
    (Variables|/Game/Project/Blueprints/Actors/Machines/BP_ForMachine.BP_ForMachine_C|SetUIInGame _array_element (Variables|Default|GetWBP_UIInGame)))
  (bind _outactors_2 (Actor|GetAllActorsOfClass "/Game/Project/Blueprints/Actors/BP_Platform.BP_Platform_C"))
  (bind _output_get_2 (Variables|Default|SetBP_Platform _outactors_2))
  (for _array_element_2 _output_get_2
    (Variables|/Game/Project/Blueprints/Actors/BP_Platform.BP_Platform_C|SetWbpuiInGAmE _array_element_2 (Variables|Default|GetWBP_UIInGame))))

(event Custom|ConstructUI
  ;[0.15 0.1473 0 0.5] MAIN
  ;;[0.15 0.15 0.15 0.5] ConstructUI
  (bind _returnvalue (Game|ConstructObjectfromClass "/Game/Project/Blueprints/UI/Widgets/WBP_UIINGame.WBP_UIINGame_C"))
  (Variables|Default|SetWBP_UIInGame _returnvalue)
  (bind _returnvalue_2 (Game|ConstructObjectfromClass "/Game/Project/Blueprints/UI/Widgets/WBP_MainMenu.WBP_MainMenu_C"))
  (Variables|Default|SetWBP_MainMenu _returnvalue_2)
  (bind _returnvalue_3 (Game|ConstructObjectfromClass "/Game/Project/Blueprints/UI/Widgets/WBP_Settings.WBP_Settings_C"))
  (Variables|Default|SetWBP_Settings _returnvalue_3)
  (bind _returnvalue_4 (Game|ConstructObjectfromClass "/Game/Project/Blueprints/UI/Widgets/WBP_Menu.WBP_Menu_C"))
  (Variables|Default|SetWBP_Menu _returnvalue_4)
  (bind _returnvalue_5 (Game|ConstructObjectfromClass "/Game/Project/Blueprints/UI/Widgets/WBP_Tutorial.WBP_Tutorial_C"))
  (Variables|Default|SetWBP_Tutorial _returnvalue_5)
  (CallFunction|MainMenuUI))

(event Custom|MainMenuUI
  ;[0.15 0.15 0.15 0.5] UI
  ;;[0.15 0.15 0.15 0.5] MainMenu
  (Viewport|RemoveAllWidgets)
  (UserInterface|Viewport|AddtoViewport (Variables|Default|GetWBP_MainMenu) 0)
  (Variables|Default|SetInGame false)
  (Variables|/Script/Engine.PlayerController|SetbShowMouseCursor (Game|GetPlayerController 0) true)
  (Utilities|FlowControl|DoOnce false
    (:Completed
      (CallFunction|Music))))

(event Custom|GameUI
  ;[0.15 0.15 0.15 0.5] UI
  ;;[0.15 0.15 0.15 0.5] Game
  (Viewport|RemoveAllWidgets)
  (UserInterface|Viewport|AddtoViewport (Variables|Default|GetWBP_UIInGame) 0)
  (Variables|Default|SetInGame true)
  (if (Audio|Components|Audio|IsPlaying (Variables|Default|GetSW_InMenu))
    (CallFunction|Music)))

(event EventBeginPlay
  ;[0.15 0.1473 0 0.5] MAIN
  ;;[0.15 0.15 0.15 0.5] EventBeginPlay
  (CallFunction|MovementTimer)
  (CallFunction|Anti-CoinsValue)
  (CallFunction|ConstructMusic)
  (CallFunction|ConstructUI)
  (CallFunction|GetActorsOfClass)
  (CallFunction|FalseUpdateSkip))

(event Input|AxisEvents|InputAxisWheel
  (params (AxisValue :type Float%20%28single-precision%29))
  (bind _returnvalue (Math|Float|Truncate AxisValue))
  ;[0.15 0.15 0.15 0.5] Movement
  (Utilities|FlowControl|Sequence
    (:then_0
      (if (== _returnvalue 1)
        (Utilities|FlowControl|Gate true) ; enters at Open
        (else
          (Utilities|FlowControl|Gate true) ; enters at Close
        )))
    (:then_1
      (if (== _returnvalue -1)
        (Utilities|FlowControl|Gate true) ; enters at Open
        (else
          (Utilities|FlowControl|Gate true) ; enters at Close
        )))))

(event Input|KeyboardEvents|A
  (params (Key :type Key%20Structure :default "None"))
  ;[0.15 0.15 0.15 0.5] Movement
  (:Pressed
    (Utilities|FlowControl|Gate true) ; enters at Open
  )
  (:Released
    (Utilities|FlowControl|Gate true) ; enters at Close
  ))

(event Input|KeyboardEvents|S
  (params (Key :type Key%20Structure :default "None"))
  ;[0.15 0.15 0.15 0.5] Movement
  (:Pressed
    (Utilities|FlowControl|Gate true) ; enters at Open
  )
  (:Released
    (Utilities|FlowControl|Gate true) ; enters at Close
  ))

(event Input|KeyboardEvents|D
  (params (Key :type Key%20Structure :default "None"))
  ;[0.15 0.15 0.15 0.5] Movement
  (:Pressed
    (Utilities|FlowControl|Gate true) ; enters at Open
  )
  (:Released
    (Utilities|FlowControl|Gate true) ; enters at Close
  ))

(event Input|MouseEvents|RightMouseButton
  (params (Key :type Key%20Structure :default "None"))
  ;[0.15 0.15 0.15 0.5] RightClickWork
  (:Pressed
    (Default|CallRightClick)))

(event Input|KeyboardEvents|W
  (params (Key :type Key%20Structure :default "None"))
  ;[0.15 0.15 0.15 0.5] Movement
  (:Pressed
    (Utilities|FlowControl|Gate true) ; enters at Open
  )
  (:Released
    (Utilities|FlowControl|Gate true) ; enters at Close
  ))

(fn ConstructionScript)

(fn ChangeCoins
  (params (CoinTypeForSubtract :type Integer) (Level :type Integer) (-Value :type Array%20of%20Integers) (+/- :type Boolean) (+Value :type Array%20of%20Integers) (CoinTypeForAdd :type Integer))
  (bind _output (Utilities|Array|Get(acopy) +Value Level))
  (bind _output_2 (Utilities|Array|Get(acopy) -Value Level))
  (if +/-
    (switch int CoinTypeForSubtract
      (:0
        (if (>= (Variables|Default|GetBronze_Coin) _output_2)
          (Variables|Default|SetBronze_Coin (- (Variables|Default|GetBronze_Coin) _output_2))
          (bind _output_get (Variables|Default|SetDone true :!label _label))
          (else
            (Variables|Default|SetDone false :!label _label_2))))
      (:1
        (if (>= (Variables|Default|GetSilver_Coin) _output_2)
          (Variables|Default|SetSilver_Coin (- (Variables|Default|GetSilver_Coin) _output_2))
          (goto _label)
          (else
            (goto _label_2))))
      (:2
        (if (>= (Variables|Default|GetGold_Coin) _output_2)
          (Variables|Default|SetGold_Coin (- (Variables|Default|GetGold_Coin) _output_2))
          (goto _label)
          (else
            (goto _label_2)))))
    (return _output_get)
    (else
      (switch int CoinTypeForAdd
        (:0
          (Variables|Default|SetBronze_Coin (+ (Variables|Default|GetBronze_Coin) _output)))
        (:1
          (Variables|Default|SetSilver_Coin (+ (Variables|Default|GetSilver_Coin) _output)))
        (:2
          (Variables|Default|SetGold_Coin (+ (Variables|Default|GetGold_Coin) _output)))))))

(fn Movement
  (params (WayOfMove :type Integer))
  (switch int WayOfMove
    (:0
      (if (not (>= (Variables|Default|GetMoveForward) 300))
        (Variables|Default|SetMoveForward (+ (Variables|Default|GetMoveForward) (Variables|Default|GetTimeForMoveForward)))
        (if (not (>= (Variables|Default|GetMoveForward) 300))
          (Utilities|FlowControl|Sequence
            (:then_0
              (Transformation|AddActorWorldOffset (Utilities|Array|Get(acopy) (Variables|Default|GetVectorOfMove) (Variables|Default|GetWayOfMove)) :!label _label))
            (:then_1
              (Variables|Default|SetMoveBackward (- (Variables|Default|GetMoveBackward) (Variables|Default|GetTimeForMoveBackward))))))))
    (:1
      (if (not (>= (Variables|Default|GetMoveBackward) 300))
        (Variables|Default|SetMoveBackward (+ (Variables|Default|GetMoveBackward) (Variables|Default|GetTimeForMoveBackward)))
        (if (not (>= (Variables|Default|GetMoveBackward) 300))
          (Utilities|FlowControl|Sequence
            (:then_1
              (Variables|Default|SetMoveForward (- (Variables|Default|GetMoveForward) (Variables|Default|GetTimeForMoveForward)))
              (goto _label))))))
    (:2
      (if (not (>= (Variables|Default|GetMoveLeft) 300))
        (Variables|Default|SetMoveLeft (+ (Variables|Default|GetMoveLeft) (Variables|Default|GetTimeForMoveLeft)))
        (if (not (>= (Variables|Default|GetMoveLeft) 300))
          (Utilities|FlowControl|Sequence
            (:then_1
              (Variables|Default|SetMoveRight (- (Variables|Default|GetMoveRight) (Variables|Default|GetTimeForMoveRight)))
              (goto _label))))))
    (:3
      (if (not (>= (Variables|Default|GetMoveRight) 300))
        (Variables|Default|SetMoveRight (+ (Variables|Default|GetMoveRight) (Variables|Default|GetTimeForMoveRight)))
        (if (not (>= (Variables|Default|GetMoveRight) 300))
          (Utilities|FlowControl|Sequence
            (:then_1
              (Variables|Default|SetMoveLeft (- (Variables|Default|GetMoveLeft) (Variables|Default|GetTimeForMoveLeft)))
              (goto _label))))))
    (:4
      (if (not (>= (Variables|Default|GetMoveDown) 100))
        (Variables|Default|SetMoveDown (+ (Variables|Default|GetMoveDown) (Variables|Default|GetTimeForMoveDown)))
        (if (not (>= (Variables|Default|GetMoveDown) 100))
          (Utilities|FlowControl|Sequence
            (:then_1
              (Variables|Default|SetMoveUp (- (Variables|Default|GetMoveUp) (Variables|Default|GetTimeForMoveUp)))
              (goto _label))))))
    (:5
      (if (not (>= (Variables|Default|GetMoveUp) 50))
        (Variables|Default|SetMoveUp (+ (Variables|Default|GetMoveUp) (Variables|Default|GetTimeForMoveUp)))
        (if (not (>= (Variables|Default|GetMoveUp) 50))
          (Utilities|FlowControl|Sequence
            (:then_1
              (Variables|Default|SetMoveDown (- (Variables|Default|GetMoveDown) (Variables|Default|GetTimeForMoveDown)))
              (goto _label))))))))