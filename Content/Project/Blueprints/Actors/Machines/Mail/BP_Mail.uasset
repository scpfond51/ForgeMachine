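; BP_Mail is a mail machine actor that opens the mail quest menu when clicked.
; A mesh click sets UpdateTarget and, unless the in-game UI's build selector is running, makes the quest menu's widgets visible.
; A separate event clears UpdateTarget when the shared update and quest menu border is hidden.
; BeginPlay caches a BP_Camera reference, which the visible logic does not use further.
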(event OnClicked(StaticMeshComponent)
  (params (TouchedComponent :type Primitive%20Component%20Object%20Reference) (ButtonPressed :type Key%20Structure :default "None"))
  (bind _wbp_uiingame (Variables|Default|GetWBP_UIInGame))
  ;[0.15 0.15 0.15 0.5] UpdateMenu
  (Variables|Default|SetUpdateTarget true)
  (if (not (Variables|/Game/Project/Blueprints/UI/Widgets/WBP_UIINGame.WBP_UIINGame_C|GetRunBuildSelector _wbp_uiingame))
    (Widget|SetVisibility (Variables|/Game/Project/Blueprints/UI/Widgets/WBP_UIINGame.WBP_UIINGame_C|GetTXT_MailQuestMenu _wbp_uiingame) "Visible")
    (Widget|SetVisibility (Variables|/Game/Project/Blueprints/UI/Widgets/WBP_UIINGame.WBP_UIINGame_C|GetT_MailQuestMenu _wbp_uiingame) "Visible")
    (Widget|SetVisibility (Variables|/Game/Project/Blueprints/UI/Widgets/WBP_UIINGame.WBP_UIINGame_C|GetB_MailQuestMenu _wbp_uiingame) "Visible")))

(event Custom|GetActorsOfClass
  ;[0.15 0.1473 0 0.5] MAIN
  ;;[0.15 0.15 0.15 0.5] GetActorsOfClass
  (bind _returnvalue (Actor|GetActorOfClass "/Game/Charapters/BP_Camera.BP_Camera_C"))
  (Variables|Default|SetBP_Camera _returnvalue))

(event Custom|IfTUpdateMenuBorderHidden,%20UpdateTarget%20=%20False
  ;[0.15 0.15 0.15 0.5] IfTUpdateMenuBorderHidden, UpdateTarget = False
  (switch Utilities|FlowControl|Switch|SwitchonESlateVisibility (Variables|/Script/UMG.Widget|GetVisibility (Variables|/Game/Project/Blueprints/UI/Widgets/WBP_UIINGame.WBP_UIINGame_C|GetT_UpdateMenuANDQuestMenuBorder (Variables|Default|GetWBP_UIInGame)))
    (:Hidden
      (Variables|Default|SetUpdateTarget false))))

(event EventBeginPlay
  ;[0.15 0.1473 0 0.5] MAIN
  ;;[0.15 0.15 0.15 0.5] EventBeginPlay
  (CallFunction|GetActorsOfClass))

(fn ConstructionScript)