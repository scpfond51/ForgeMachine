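; BP_Mail is a clickable mailbox actor that offers random coin-trade, donation and gamble quests, with Russian text shown in the in-game UI.
; Hovering outlines the mesh, clicking squashes it, and right-clicking opens the mail quest menu.
; A random-delay timer picks a quest and snapshots the requested coin balance.
; Accepting opens a Gate on a polling timer, which pays out through BP_Camera once enough new coins accumulate, using resettable DoOnce guards, then schedules another.
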(event OnBeginCursorOver(StaticMeshComponent)
  (params (TouchedComponent :type Primitive%20Component%20Object%20Reference))
  ;[0.15 0.15 0.15 0.5] UpdateMenu
  (Variables|Default|SetOnComponent true)
  (Rendering|Material|SetOverlayMaterial (Variables|Debug|GetStaticMeshComponent) "/Game/Project/MaterialLibrary/Materials/M_Outline.M_Outline" :!class /Script/Engine.MeshComponent))

(event OnEndCursorOver(StaticMeshComponent)
  (params (TouchedComponent :type Primitive%20Component%20Object%20Reference))
  ;[0.15 0.15 0.15 0.5] UpdateMenu
  (Variables|Default|SetOnComponent false)
  (Rendering|Material|SetOverlayMaterial (Variables|Debug|GetStaticMeshComponent) 0 :!class /Script/Engine.MeshComponent))

(event OnClicked(StaticMeshComponent)
  (params (TouchedComponent :type Primitive%20Component%20Object%20Reference) (ButtonPressed :type Key%20Structure :default "None"))
  ;[0.15 0.15 0.15 0.5] Effects
  (Utilities|ClickAnimation))

(event Custom|UpdateMenu
  (bind _wbp_uiingame (Variables|Default|GetWBP_UIInGame))
  ;[0.15 0.15 0.15 0.5] UpdateMenu
  (if (Variables|Default|GetOnComponent)
    (Utilities|FlowControl|Sequence
      (:then_0
        (Variables|Default|SetUpdateTarget true)
        (if (not (Variables|/Game/Project/Blueprints/UI/Widgets/WBP_UIINGame.WBP_UIINGame_C|GetRunBuildSelector _wbp_uiingame))
          (Widget|SetVisibility (Variables|/Game/Project/Blueprints/UI/Widgets/WBP_UIINGame.WBP_UIINGame_C|GetTXT_MailQuestMenu _wbp_uiingame) "Visible")
          (Widget|SetVisibility (Variables|/Game/Project/Blueprints/UI/Widgets/WBP_UIINGame.WBP_UIINGame_C|GetT_MailQuestMenu _wbp_uiingame) "Visible")
          (Widget|SetVisibility (Variables|/Game/Project/Blueprints/UI/Widgets/WBP_UIINGame.WBP_UIINGame_C|GetB_MailQuestMenu _wbp_uiingame) "Visible")))
      (:then_1
        (Utilities|ClickAnimation)))))

(event Custom|Quest
  (AddComponent|AddAudioComponent false)
  (switch int (Math|Random|RandomIntegerinRange 1 6)
    (:1
      (CallFunction|SetText "Незнакомец - \"Эй, привет! Я хотел попросить у вас ну... Скажем... 1000 медных монет, ой... Нет, простите 2500 медных монет. 
Мне просто нужна еда, а серебряные монеты не принимают из-за того, что они слишком крупные. Я дам вам 100 серебряных, гарантирую!\"")
      (CallFunction|SaveOLDCoinsandChangeValue 2500)
      (CallFunction|ResetDoOnce)
      (Variables|Default|SetNumberOfAcceptedQuest 1))
    (:2
      (CallFunction|SetText "Оу, прииувееет!... *Ик* Я вот хочу тебе предложить... НУ Знаешь, медь!... Хех... В общем!.. Мгх.. Прости, я сегодня оооочень пьян 
Ну в общем! Скажем 5 золотых монет и 5000 меди твои! Скажешь зачем? Мне выпивка нужна, не более. Ну давааай же, я потом отстану...")
      (CallFunction|SaveOLDCoinsandChangeValue 5 2)
      (CallFunction|ResetDoOnce)
      (Variables|Default|SetNumberOfAcceptedQuest 2))
    (:3
      (CallFunction|SetText "Физкульт привет, не буду томить, я хочу купить оружия. Да-да, знаю, вы не производите оружие, но... Я хочу обменяться. 
За золотые монеты, можно возобновить производство оружия, которое было уничтожено... А воякам пригодилось бы пару сотен пушек 
Итак, предлагаю тебе 10000 серебряных монет, взамен - ты мне даёшь 20 золотых, идёт?")
      (CallFunction|SaveOLDCoinsandChangeValue 20 2)
      (CallFunction|ResetDoOnce)
      (Variables|Default|SetNumberOfAcceptedQuest 3))
    (:4
      (CallFunction|SetText "Фух! Еле добрался! Друг, мне нужна твоя помощь, иначе я в провале. Вся поставка груза уничтожена. НАМ СРОЧНО НУЖНО СЕРЕБРО!! 
500 нет.. 1000... Нет... 30000 серебра! 30000 СЕРЕБРА!!! Я потом тебе отплачу, награда будет высокой, не переживай. У нас 3 с половиной минуты")
      (CallFunction|SaveOLDCoinsandChangeValue 30000 1)
      (CallFunction|ResetDoOnce)
      (Variables|Default|SetNumberOfAcceptedQuest 4))
    (:5
      (CallFunction|SetText "П-простите... В-вы поддерживаете право деревьям жить? Ой, эм... Вы.. Хотите... Б-блин, забываю... Не хотите поддержать наш проект 
по защите природы? Мм.. Ну... 1000 серебра")
      (CallFunction|SaveOLDCoinsandChangeValue 1000 1)
      (CallFunction|ResetDoOnce)
      (Variables|Default|SetNumberOfAcceptedQuest 5))
    (:6
      (CallFunction|SetText "Привет-привет! Тебе только что улыбнулась удача, ты можешь обогатиться и разориться в одно мгновение! Заплати мне 100 золота, и возможно ты 
получишь в 2 раза больше 
")
      (CallFunction|SaveOLDCoinsandChangeValue 100 2)
      (CallFunction|ResetDoOnce)
      (Variables|Default|SetNumberOfAcceptedQuest 6))))

(event Custom|InitStuff
  (Utilities|FlowControl|Sequence
    (:then_0
      (EventDispatchers|BindEventtoQuestButtons (Variables|Default|GetWBP_UIInGame) (delegate Custom|Questchange)))
    (:then_1
      (Utilities|Time|SetTimerbyEvent (delegate Custom|Coins) 0.1 true))))

(event Custom|ChangeEffectVisibility
  (bind _staticmeshcomponent (Variables|Debug|GetStaticMeshComponent))
  ;[0.15 0.15 0.15 0.5] Effects
  (if (Variables|/Game/Charapters/BP_Camera.BP_Camera_C|GetEffect (Variables|Default|GetBP_Camera))
    (Rendering|Material|SetOverlayMaterial _staticmeshcomponent 0 :!class /Script/Engine.MeshComponent)
    (else
      (Rendering|Material|SetOverlayMaterial _staticmeshcomponent "/Game/Project/MaterialLibrary/Materials/M_Outline.M_Outline" :!class /Script/Engine.MeshComponent))))

(event Custom|Effects
  ;[0.15 0.15 0.15 0.5] Effects
  (EventDispatchers|BindEventtoEDEffects (Variables|Default|GetBP_Camera) (delegate Custom|ChangeEffectVisibility)))

(event Custom|CoinsTimer
  (Utilities|FlowControl|Gate true) ; enters at Toggle
)

(event Custom|Coins
  (Utilities|FlowControl|Gate true
    (:Exit
      (switch int (Variables|Default|GetNumberOfAcceptedQuest)
        (:1
          (bind _returnvalue (Utilities|Coins-OldValueCoins=Value (Variables|/Game/Charapters/BP_Camera.BP_Camera_C|GetBronze_Coin (Variables|Default|GetBP_Camera)))
            (:NewParam2
              (if _returnvalue
                (Utilities|FlowControl|DoOnce false
                  (:Completed
                    (CallFunction|CoinTypetoAdd/Subtract,andTheirLevel 0 1)
                    (Default|ChangeCoins (Variables|Default|GetBP_Camera) (Variables|Default|GetCoinTypeToSubtract) (Variables|Default|Getlevel) (Variables|Default|Get-%20Value) true :!label _label)
                    (Default|ChangeCoins (Variables|Default|GetBP_Camera) 0 (Variables|Default|Getlevel) 0 false (Variables|Default|Get+%20Value) (Variables|Default|GetCoinTypeToAdd))
                    (if (Variables|Default|GetAgainAdd)
                      (Default|ChangeCoins (Variables|Default|GetBP_Camera) 0 0 0 false (Variables|Default|Get+%20Value2) (Variables|Default|GetCoinTypeToAdd2))
                      (Variables|Default|SetAgainAdd false))
                    (CallFunction|SetText "Задание выполнено" :!label _label_2)
                    (CallFunction|CoinsTimer)
                    (CallFunction|ResetQuestValues)
                    (CallFunction|QuestTimerandEvent)))))))
        (:2
          (bind _returnvalue_2 (Utilities|Coins-OldValueCoins=Value (Variables|/Game/Charapters/BP_Camera.BP_Camera_C|GetGold_Coin (Variables|Default|GetBP_Camera)))
            (:NewParam2
              (if _returnvalue_2
                (Utilities|FlowControl|DoOnce false
                  (:Completed
                    (CallFunction|CoinTypetoAdd/Subtract,andTheirLevel 2 0 1)
                    (goto _label)))))))
        (:3
          (bind _returnvalue_3 (Utilities|Coins-OldValueCoins=Value (Variables|/Game/Charapters/BP_Camera.BP_Camera_C|GetGold_Coin (Variables|Default|GetBP_Camera)))
            (:NewParam2
              (if _returnvalue_3
                (Utilities|FlowControl|DoOnce false
                  (:Completed
                    (CallFunction|CoinTypetoAdd/Subtract,andTheirLevel 2 1 2)
                    (goto _label)))))))
        (:4
          (bind _returnvalue_4 (Utilities|Coins-OldValueCoins=Value (Variables|/Game/Charapters/BP_Camera.BP_Camera_C|GetSilver_Coin (Variables|Default|GetBP_Camera)))
            (:NewParam2
              (if _returnvalue_4
                (Utilities|FlowControl|DoOnce false
                  (:Completed
                    (CallFunction|CoinTypetoAdd/Subtract,andTheirLevel 1 2 3)
                    (Variables|Default|SetCoinTypeToAdd2 3)
                    (Variables|Default|SetAgainAdd true)
                    (goto _label)))))))
        (:5
          (bind _returnvalue_5 (Utilities|Coins-OldValueCoins=Value (Variables|/Game/Charapters/BP_Camera.BP_Camera_C|GetSilver_Coin (Variables|Default|GetBP_Camera)))
            (:NewParam2
              (if _returnvalue_5
                (Utilities|FlowControl|DoOnce false
                  (:Completed
                    (bind _done (Default|ChangeCoins (Variables|Default|GetBP_Camera) 1 4 (Variables|Default|Get-%20Value) true))
                    (if _done
                      (goto _label_2))))))))
        (:6
          (bind _returnvalue_6 (Utilities|Coins-OldValueCoins=Value (Variables|/Game/Charapters/BP_Camera.BP_Camera_C|GetGold_Coin (Variables|Default|GetBP_Camera)))
            (:NewParam2
              (if _returnvalue_6
                (Utilities|FlowControl|DoOnce false
                  (:Completed
                    (bind _done_2 (Default|ChangeCoins (Variables|Default|GetBP_Camera) 2 5 (Variables|Default|Get-%20Value) true))
                    (if _done_2
                      (if (>= (Math|Random|RandomIntegerinRange 0 100) 50)
                        (CallFunction|SetText "Не повезло")
                        (else
                          (Default|ChangeCoins (Variables|Default|GetBP_Camera) 0 4 0 false (Variables|Default|Get+%20Value) 2)
                          (CallFunction|SetText "Повезло, +250 золота")))
                      (CallFunction|CoinsTimer)
                      (CallFunction|ResetQuestValues)
                      (CallFunction|QuestTimerandEvent))))))))))))

(event Custom|GetActorsOfClass
  ;[0.15 0.1473 0 0.5] MAIN
  ;;[0.15 0.15 0.15 0.5] GetActorsOfClass
  (bind _returnvalue (Actor|GetActorOfClass "/Game/Charapters/BP_Camera.BP_Camera_C"))
  (Variables|Default|SetBP_Camera _returnvalue))

(event Custom|UpdateMenuBeginPlay
  ;[0.15 0.15 0.15 0.5] UpdateMenu
  (EventDispatchers|BindEventtoRightClick (Variables|Default|GetBP_Camera) (delegate Custom|UpdateMenu)))

(event Custom|ResetDoOnce
  (Utilities|FlowControl|Sequence
    (:then_0
      (Utilities|FlowControl|DoOnce false) ; enters at Reset
    )
    (:then_1
      (Utilities|FlowControl|Sequence
        (:then_0
          (Utilities|FlowControl|DoOnce false) ; enters at Reset
        )
        (:then_1
          (Utilities|FlowControl|DoOnce false) ; enters at Reset
        )
        (:then_2
          (Utilities|FlowControl|DoOnce false) ; enters at Reset
        )
        (:then_3
          (Utilities|FlowControl|DoOnce false) ; enters at Reset
        )
        (:then_4
          (Utilities|FlowControl|DoOnce false) ; enters at Reset
        )
        (:then_5
          (Utilities|FlowControl|DoOnce false) ; enters at Reset
        )))))

(event Custom|QuestTimerAndEvent
  (Utilities|Time|SetTimerbyEvent (delegate Custom|Quest) (Math|Conversions|ToFloat(Integer) (Math|Random|RandomIntegerinRange 10 20))))

(event Custom|Questchange
  (params (Accepted :type Boolean))
  (Utilities|FlowControl|DoOnce false
    (:Completed
      (if Accepted
        (CallFunction|CoinsTimer)
        (else
          (CallFunction|SetText "Отказ от задания")
          (CallFunction|ResetQuestValues)
          (CallFunction|QuestTimerandEvent))))))

(event Custom|IfTUpdateMenuBorderHidden,%20UpdateTarget%20=%20False
  ;[0.15 0.15 0.15 0.5] IfTUpdateMenuBorderHidden, UpdateTarget = False
  (switch Utilities|FlowControl|Switch|SwitchonESlateVisibility (Variables|/Script/UMG.Widget|GetVisibility (Variables|/Game/Project/Blueprints/UI/Widgets/WBP_UIINGame.WBP_UIINGame_C|GetT_UpdateMenuANDQuestMenuBorder (Variables|Default|GetWBP_UIInGame)))
    (:Hidden
      (Variables|Default|SetUpdateTarget false))))

(event EventBeginPlay
  ;[0.15 0.1473 0 0.5] MAIN
  ;;[0.15 0.15 0.15 0.5] EventBeginPlay
  (CallFunction|GetActorsOfClass)
  (CallFunction|UpdateMenuBeginPlay)
  (CallFunction|InitStuff)
  (CallFunction|QuestTimerandEvent)
  (CallFunction|Effects))

(fn ConstructionScript)

(fn SetText
  (params (Text :type Text))
  (Variables|/Script/UMG.TextBlock|SetText (Variables|/Game/Project/Blueprints/UI/Widgets/WBP_UIINGame.WBP_UIINGame_C|GetTXT_UpdateMenuQuest (Variables|Default|GetWBP_UIInGame)) Text))

(fn SaveOLDCoinsandChangeValue
  (params (Value :type Integer) (CoinType :type Integer))
  (bind _bp_camera (Variables|Default|GetBP_Camera))
  (Variables|Default|SetValue Value)
  (switch int CoinType
    (:0
      (Variables|Default|SetOldValueCoins (Variables|/Game/Charapters/BP_Camera.BP_Camera_C|GetBronze_Coin _bp_camera)))
    (:1
      (Variables|Default|SetOldValueCoins (Variables|/Game/Charapters/BP_Camera.BP_Camera_C|GetSilver_Coin _bp_camera)))
    (:2
      (Variables|Default|SetOldValueCoins (Variables|/Game/Charapters/BP_Camera.BP_Camera_C|GetGold_Coin _bp_camera)))))

(fn CoinTypetoAdd/Subtract,andTheirLevel
  (params (CoinTypeSubtract :type Integer) (CoinTypeToAdd :type Integer) (level :type Integer))
  (Variables|Default|SetCoinTypeToSubtract CoinTypeSubtract)
  (Variables|Default|SetCoinTypeToAdd CoinTypeToAdd)
  (Variables|Default|Setlevel level))

(fn ResetQuestValues
  (Variables|Default|SetNumberOfAcceptedQuest 0)
  (Variables|Default|SetOldValueCoins 0)
  (Variables|Default|SetValue 0)
  (Variables|Default|SetCoinTypeToSubtract 0)
  (Variables|Default|SetCoinTypeToAdd 0)
  (Variables|Default|Setlevel 0))