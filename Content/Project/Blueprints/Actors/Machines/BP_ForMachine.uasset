(event Custom|Timer
  (bind _bp_battery (Variables|Default|GetBP_Battery))
  (bind _bp_lamp (Variables|Default|GetBP_Lamp))
  (bind _bp_largebattery (Variables|Default|GetBP_LargeBattery))
  (bind _bp_sage (Variables|Default|GetBP_Sage))
  (if (Variables|Default|GetStop)
    (Utilities|FlowControl|DoOnce false :!label _label
      (:Completed
        (CallFunction|Sound)))
    (else
      (Utilities|FlowControl|Sequence
        (:then_0
          (goto _label Reset))
        (:then_1
          ;[0.15 0.15 0.15 0.5] PreSpawn
          (Utilities|FlowControl|Delay 0.2)
          (CallFunction|PreSpawn (Variables|/Game/Project/Blueprints/UI/Widgets/WBP_UIINGame.WBP_UIINGame_C|GetMachineNumber (Variables|Default|GetUIInGame))))
        (:then_2
          ;[0.15 0.15 0.15 0.5] Spawn
          (Utilities|FlowControl|Delay 0.2)
          (CallFunction|Spawn (Variables|/Game/Project/Blueprints/UI/Widgets/WBP_UIINGame.WBP_UIINGame_C|GetMachineNumber (Variables|Default|GetUIInGame)) (stale Custom|SaveBuilded SaveBuilded))
          ;[0.15 0.15 0.15 0.5] DestroyActorBySell
          (Utilities|IsValid _bp_battery
            (:Is%20Valid
              (EventDispatchers|BindEventtoDestroyed _bp_battery (delegate Custom|DestroyedBattery)))
            (:Is%20Not%20Valid
              _))
          (Utilities|IsValid _bp_lamp
            (:Is%20Valid
              (EventDispatchers|BindEventtoDestroyed _bp_lamp (delegate Custom|DestroyedLamp)))
            (:Is%20Not%20Valid
              _))
          (Utilities|IsValid _bp_largebattery
            (:Is%20Valid
              (EventDispatchers|BindEventtoDestroyed _bp_largebattery (delegate Custom|DestroyedLargeBattery)))
            (:Is%20Not%20Valid
              _))
          (Utilities|IsValid _bp_sage
            (:Is%20Valid
              (EventDispatchers|BindEventtoDestroyed _bp_sage (delegate Custom|DestroyedSafe)))))))))

(event Custom|DestroyedBattery
  ;[0.15 0.15 0.15 0.5] DestroyActorBySell
  (Variables|Default|SetBP_Battery 0)
  (Variables|Default|SetStop false)
  (Variables|Default|SetBuilded false))

(event Custom|DestroyedSafe
  ;[0.15 0.15 0.15 0.5] DestroyActorBySell
  (Variables|Default|SetBP_Lamp 0)
  (Variables|Default|SetStop false)
  (Variables|Default|SetBuilded false))

(event Custom|DestroyedLamp
  ;[0.15 0.15 0.15 0.5] DestroyActorBySell
  (Variables|Default|SetBP_Lamp 0)
  (Variables|Default|SetStop false)
  (Variables|Default|SetBuilded false))

(event Custom|Sound
  ;[0.15 0.15 0.15 0.5] Sound
  (Default|Sounds (Variables|Default|GetBP_Camera) true false false))

(event Custom|DestroyedLargeBattery
  ;[0.15 0.15 0.15 0.5] DestroyActorBySell
  (Variables|Default|SetBP_Lamp 0)
  (Variables|Default|SetStop false)
  (Variables|Default|SetBuilded false))

(event Custom|SaveBuilded
  (params (SaveBuilded :type Boolean))
  (bind _bp_battery (Variables|Default|GetBP_Battery))
  (bind _bp_lamp (Variables|Default|GetBP_Lamp))
  (bind _bp_largebattery (Variables|Default|GetBP_LargeBattery))
  (bind _bp_sage (Variables|Default|GetBP_Sage))
  ;[0.15 0.15 0.15 0.5] Spawn
  (CallFunction|Spawn (Variables|/Game/Project/Blueprints/UI/Widgets/WBP_UIINGame.WBP_UIINGame_C|GetMachineNumber (Variables|Default|GetUIInGame)) SaveBuilded)
  ;[0.15 0.15 0.15 0.5] DestroyActorBySell
  (Utilities|IsValid _bp_battery
    (:Is%20Valid
      (EventDispatchers|BindEventtoDestroyed _bp_battery (delegate Custom|DestroyedBattery)))
    (:Is%20Not%20Valid
      _))
  (Utilities|IsValid _bp_lamp
    (:Is%20Valid
      (EventDispatchers|BindEventtoDestroyed _bp_lamp (delegate Custom|DestroyedLamp)))
    (:Is%20Not%20Valid
      _))
  (Utilities|IsValid _bp_largebattery
    (:Is%20Valid
      (EventDispatchers|BindEventtoDestroyed _bp_largebattery (delegate Custom|DestroyedLargeBattery)))
    (:Is%20Not%20Valid
      _))
  (Utilities|IsValid _bp_sage
    (:Is%20Valid
      (EventDispatchers|BindEventtoDestroyed _bp_sage (delegate Custom|DestroyedSafe)))))

(event EventBeginPlay
  (bind _returnvalue (Actor|GetActorOfClass "/Game/Charapters/BP_Camera.BP_Camera_C"))
  (Variables|Default|SetBP_Camera _returnvalue)
  (Utilities|Time|SetTimerbyEvent (delegate Custom|Timer) 0.05 true))

(fn ConstructionScript)

(fn PreSpawn
  (params (MachineNumber :type Integer))
  (bind _cursoronplatform (Variables|Default|GetCursorOnPlatform))
  (bind _staticmesh (Variables|Default|GetStaticMesh))
  (bind _cursoronplatform_2 (Variables|Default|GetCursorOnPlatform))
  (bind _staticmesh_2 (Variables|Default|GetStaticMesh))
  (bind _cursoronplatform_3 (Variables|Default|GetCursorOnPlatform))
  (bind _staticmesh_3 (Variables|Default|GetStaticMesh))
  (bind _cursoronplatform_4 (Variables|Default|GetCursorOnPlatform))
  (bind _staticmesh_4 (Variables|Default|GetStaticMesh))
  (bind _cursoronplatform_5 (Variables|Default|GetCursorOnPlatform))
  (bind _staticmesh_5 (Variables|Default|GetStaticMesh))
  (bind _cursoronplatform_6 (Variables|Default|GetCursorOnPlatform))
  (bind _staticmesh_6 (Variables|Default|GetStaticMesh))
  (switch int MachineNumber
    (:1
      (if _cursoronplatform
        _
        (else
          _))
      (Components|StaticMesh|SetStaticMesh _staticmesh "/Game/Project/MaterialLibrary/Meshes/Big_boy.Big_boy")
      (Rendering|SetVisibility _staticmesh _cursoronplatform false))
    (:2
      (if _cursoronplatform_3
        _
        (else
          _))
      (Components|StaticMesh|SetStaticMesh _staticmesh_3 "/Game/Project/MaterialLibrary/Meshes/Seif.Seif")
      (Rendering|SetVisibility _staticmesh_3 _cursoronplatform_3 false))
    (:3
      (if _cursoronplatform_5
        _
        (else
          _))
      (Components|StaticMesh|SetStaticMesh _staticmesh_5 "/Game/Project/MaterialLibrary/Meshes/lampa.lampa")
      (Rendering|SetVisibility _staticmesh_5 _cursoronplatform_5 false))
    (:4
      (if _cursoronplatform_6
        _
        (else
          _))
      (Components|StaticMesh|SetStaticMesh _staticmesh_6 "/Game/Project/MaterialLibrary/Meshes/Pochta.Pochta")
      (Rendering|SetVisibility _staticmesh_6 _cursoronplatform_6 false))
    (:5
      (if _cursoronplatform_2
        _
        (else
          _))
      (Components|StaticMesh|SetStaticMesh _staticmesh_2 "/Game/Project/MaterialLibrary/Meshes/Large_Battery4.Large_Battery4")
      (Rendering|SetVisibility _staticmesh_2 _cursoronplatform_2 false))
    (:6
      (if _cursoronplatform_4
        _
        (else
          _))
      (Components|StaticMesh|SetStaticMesh _staticmesh_4 "/Game/Project/MaterialLibrary/Meshes/Stanok2.Stanok2")
      (Rendering|SetVisibility _staticmesh_4 _cursoronplatform_4 false))))

(fn Spawn
  (params (MachineNumber :type Integer) (SaveBuilded :type Boolean))
  (bind _uiingame (Variables|Default|GetUIInGame))
  (if SaveBuilded
    (switch int (Variables|Default|GetWhatBuilded)
      (:1
        (bind _returnvalue (Game|SpawnActorfromClass "/Game/Project/Blueprints/Actors/Machines/Battarey/BP_Battery.BP_Battery_C" (Transformation|GetActorTransform) "Undefined" "MultiplyWithRoot" 0 0 :!label _label))
        (Variables|/Game/Project/Blueprints/Actors/Machines/Battarey/BP_Battery.BP_Battery_C|SetWBP_UIInGame _returnvalue (Variables|Default|GetUIInGame))
        (Variables|Default|SetBP_Battery _returnvalue)
        (Variables|Default|SetWhatBuilded 1))
      (:2
        (bind _returnvalue_2 (Game|SpawnActorfromClass "/Game/Project/Blueprints/Actors/Machines/Safe/BP_Safe.BP_Safe_C" (Transformation|GetActorTransform) "Undefined" "MultiplyWithRoot" 0 0 :!label _label_2))
        (Variables|/Game/Project/Blueprints/Actors/Machines/Safe/BP_Safe.BP_Safe_C|SetWBP_UIInGame _returnvalue_2 (Variables|Default|GetUIInGame))
        (Variables|Default|SetBP_Sage _returnvalue_2)
        (Variables|Default|SetWhatBuilded 2))
      (:3
        (bind _returnvalue_3 (Game|SpawnActorfromClass "/Game/Project/Blueprints/Actors/Machines/Lampa/BP_Lamp.BP_Lamp_C" (Transformation|GetActorTransform) "Undefined" "MultiplyWithRoot" 0 0 :!label _label_3))
        (Variables|/Game/Project/Blueprints/Actors/Machines/Lampa/BP_Lamp.BP_Lamp_C|SetWBP_UIInGame _returnvalue_3 (Variables|Default|GetUIInGame))
        (Variables|Default|SetBP_Lamp _returnvalue_3)
        (Variables|Default|SetWhatBuilded 3))
      (:4
        (bind _returnvalue_4 (Game|SpawnActorfromClass "/Game/Project/Blueprints/Actors/Machines/Mail/BP_Mail.BP_Mail_C" (Transformation|GetActorTransform) "Undefined" "MultiplyWithRoot" 0 0 :!label _label_4))
        (Variables|/Game/Project/Blueprints/Actors/Machines/Mail/BP_Mail.BP_Mail_C|SetWBP_UIInGame _returnvalue_4 (Variables|Default|GetUIInGame))
        (Variables|Default|SetBP_Mail _returnvalue_4)
        (Variables|Default|SetWhatBuilded 4))
      (:5
        (bind _returnvalue_5 (Game|SpawnActorfromClass "/Game/Project/Blueprints/Actors/Machines/LargeBattery/BP_LargeBattery.BP_LargeBattery_C" (Transformation|GetActorTransform) "Undefined" "MultiplyWithRoot" 0 0 :!label _label_5))
        (Variables|/Game/Project/Blueprints/Actors/Machines/LargeBattery/BP_LargeBattery.BP_LargeBattery_C|SetWBP_UIInGame _returnvalue_5 (Variables|Default|GetUIInGame))
        (Variables|Default|SetBP_LargeBattery _returnvalue_5)
        (Variables|Default|SetWhatBuilded 5))
      (:6
        (bind _returnvalue_6 (Game|SpawnActorfromClass "/Game/Project/Blueprints/Actors/Machines/Machine-1/Machine-1.Machine-1_C" (Transformation|GetActorTransform) "Undefined" "MultiplyWithRoot" 0 0 :!label _label_6))
        (Variables|/Game/Project/Blueprints/Actors/Machines/Machine-1/Machine-1.Machine-1_C|SetWBP_UIInGame _returnvalue_6 (Variables|Default|GetUIInGame))
        (Variables|Default|SetWhatBuilded 6)))
    (Variables|Default|SetBuilded false)
    (Variables|/Game/Project/Blueprints/UI/Widgets/WBP_UIINGame.WBP_UIINGame_C|SetMachineNumber _uiingame 0)
    (Variables|Default|SetStop true)
    (Default|SetVisibilityAll _uiingame "Visible" "SelfHitTestInvisible")
    (Default|SetVisibilityMenu _uiingame "Collapsed")
    (Components|StaticMesh|SetStaticMesh (Variables|Default|GetStaticMesh) 0)
    (return)
    (else
      (switch int MachineNumber
        (:1
          (if (Variables|Default|GetBuilded)
            (goto _label)))
        (:2
          (if (Variables|Default|GetBuilded)
            (goto _label_2)))
        (:3
          (if (Variables|Default|GetBuilded)
            (goto _label_3)))
        (:4
          (if (Variables|Default|GetBuilded)
            (goto _label_4)))
        (:5
          (if (Variables|Default|GetBuilded)
            (goto _label_5)))
        (:6
          (if (Variables|Default|GetBuilded)
            (goto _label_6)))))))