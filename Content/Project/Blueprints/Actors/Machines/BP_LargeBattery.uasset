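; Large battery machine actor that periodically earns coins for the player and can be upgraded or sold.
; A looping timer pays out through BP_Camera, with coin type set by Level (max 5).
; Right-click while hovered opens the shared update menu, and a 0.1-second timer polls its Upgrade and Sell flags, with selling refunding build and upgrade costs.
; BP_Camera dispatchers also drive effect visibility and machine volume.
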(event OnBeginCursorOver(StaticMeshComponent)
  (params (TouchedComponent :type Primitive%20Component%20Object%20Reference))
  ;[0.15 0.15 0.15 0.5] UpdateMenu
  (Variables|Default|SetOnComponent true)
  (Rendering|Material|SetOverlayMaterial (Variables|Debug|GetStaticMeshComponent) "/Game/Project/MaterialLibrary/Materials/M_Outline.M_Outline" :!class /Script/Engine.MeshComponent))

(event OnEndCursorOver(StaticMeshComponent)
  (params (TouchedComponent :type Primitive%20Component%20Object%20Reference))
  ;[0.15 0.15 0.15 0.5] UpdateMenu
  (Variables|Default|SetOnComponent false)
  (Rendering|Material|SetOverlayMaterial (Variables|Debug|GetStaticMeshComponent) 0 :!class /Script/Engine.MeshComponent))

(event OnClicked(StaticMeshComponent)
  (params (TouchedComponent :type Primitive%20Component%20Object%20Reference) (ButtonPressed :type Key%20Structure :default "None"))
  ;[0.15 0.15 0.15 0.5] Effects
  (Utilities|ClickAnimation))

(event Custom|UpdateMenu
  (bind _wbp_uiingame (Variables|Default|GetWBP_UIInGame))
  ;[0.15 0.15 0.15 0.5] UpdateMenu
  (if (Variables|Default|GetOnComponent)
    (Variables|Default|SetUpdateTarget true)
    (Utilities|FlowControl|Sequence
      (:then_0
        (if (not (Variables|/Game/Project/Blueprints/UI/Widgets/WBP_UIINGame.WBP_UIINGame_C|GetRunBuildSelector _wbp_uiingame))
          (Widget|SetVisibility (Variables|/Game/Project/Blueprints/UI/Widgets/WBP_UIINGame.WBP_UIINGame_C|GetTextUpdateMenu _wbp_uiingame) "Visible")
          (Widget|SetVisibility (Variables|/Game/Project/Blueprints/UI/Widgets/WBP_UIINGame.WBP_UIINGame_C|GetButtonUpdateMenu _wbp_uiingame) "Visible")
          (Widget|SetVisibility (Variables|/Game/Project/Blueprints/UI/Widgets/WBP_UIINGame.WBP_UIINGame_C|GetTexuresUpdateMenu _wbp_uiingame) "Visible")))
      (:then_1
        (Utilities|ClickAnimation)))))

(event Custom|Updatetimer
  ;[0.15 0.1473 0 0.5] MAIN
  ;;[0.15 0.15 0.15 0.5] Events
  (Utilities|FlowControl|Sequence
    (:then_0
      (if (Variables|Default|GetUpdateTarget)
        (CallFunction|ChangeUpdateMenuCoin)
        (CallFunction|ChangeDescriptionOfUpdateMenu)
        (CallFunction|CoinBackSystembySell)
        (CallFunction|UpdateTextCost)
        (CallFunction|Upgrade)))
    (:then_1
      (CallFunction|IfTUpdateMenuBorderHidden,UpdateTarget=False))))

(event Custom|leevent
  ;[0.15 0.15 0.15 0.5] ProfitFromLevel
  (switch int (Variables|Default|GetLevel)
    (:0
      (Variables|Default|SetCoinTypeForAdd 1))
    (:1
      (Variables|Default|SetCoinTypeForAdd 2 :!label _label))
    (:2
      (goto _label))
    (:3
      (goto _label))
    (:4
      (goto _label))
    (:5
      (goto _label)))
  (Default|ChangeCoins (Variables|Default|GetBP_Camera) 0 (Variables|Default|GetLevel) 0 false (Variables|Default|GetProfit) (Variables|Default|GetCoinTypeForAdd))
  (CallFunction|Sounds false false))

(event Custom|UpdateTextCost
  (bind _level (Variables|Default|GetLevel))
  (bind _wbp_uiingame (Variables|Default|GetWBP_UIInGame))
  (bind _txt_costofupdate (Variables|/Game/Project/Blueprints/UI/Widgets/WBP_UIINGame.WBP_UIINGame_C|GetTXT_CostOfUpdate _wbp_uiingame))
  ;[0.15 0.15 0.15 0.5] UpdateTextCost
  (if (== _level 5)
    (Rendering|Components|TextRender|SetText _txt_costofupdate "MAX")
    (else
      (Rendering|Components|TextRender|SetText _txt_costofupdate (Utilities|Text|ToText(Integer) (Utilities|Array|Get(acopy) (Variables|Default|GetCostOfUpdate) _level))))))

(event Custom|Upgrade
  (bind _wbp_uiingame (Variables|Default|GetWBP_UIInGame))
  ;[0.15 0.15 0.15 0.5] Upgrade
  (if (Variables|/Game/Project/Blueprints/UI/Widgets/WBP_UIINGame.WBP_UIINGame_C|GetUpdateCliked (Variables|Default|GetWBP_UIInGame))
    (if (< (Variables|Default|GetLevel) 5)
      (switch int (Variables|Default|GetLevel)
        (:0
          (bind _output_get (Variables|Default|SetCoinTypeForSubtract 1))
          (Default|ChangeUpdateMenuCoin _wbp_uiingame _output_get))
        (:1
          (bind _output_get_2 (Variables|Default|SetCoinTypeForSubtract 2 :!label _label))
          (Default|ChangeUpdateMenuCoin _wbp_uiingame _output_get_2))
        (:2
          (goto _label))
        (:3
          (goto _label))
        (:4
          (goto _label))
        (:5
          (goto _label)))
      (bind _done (Default|ChangeCoins (Variables|Default|GetBP_Camera) (Variables|Default|GetCoinTypeForSubtract) (Variables|Default|GetLevel) (Variables|Default|GetCostOfUpdate) true))
      (if _done
        (Variables|/Game/Project/Blueprints/UI/Widgets/WBP_UIINGame.WBP_UIINGame_C|SetUpdateCliked (Variables|Default|GetWBP_UIInGame) false)
        (CallFunction|UpdateCostGainforSell)
        (CallFunction|Sounds false true)
        (Variables|Default|SetLevel (+ (Variables|Default|GetLevel) 1))
        (else
          (Default|Sounds (Variables|Default|GetBP_Camera) false false false false false true))))))

(event Custom|Sounds
  (params (Selling :type Boolean) (Upgrade :type Boolean))
  ;[0.15 0.15 0.15 0.5] Sounds
  (if (or Selling Upgrade)
    (Default|Sounds (Variables|Default|GetBP_Camera) false false Selling false Upgrade false)
    (else
      (Audio|Components|Audio|Play (Variables|Default|GetSW_BigBatteryFinishedProduction) 0.0))))

(event Custom|SoundConstructions
  ;[0.15 0.1473 0 0.5] MAIN
  ;;[0.15 0.15 0.15 0.5] SoundConstructions
  (EventDispatchers|BindEventtoEDSoundMachineVolume (Variables|Default|GetBP_Camera) (delegate Custom|ChangeVolume))
  (Audio|Components|Audio|SetVolumeMultiplier (Variables|Default|GetSW_BigBatteryFinishedProduction) (Variables|Default|GetSoundMachineVolume) :!class /Script/Engine.AudioComponent))

(event Custom|StartTimer
  ;[0.15 0.15 0.15 0.5] ProfitFromLevel
  (Utilities|Time|SetTimerbyEvent (delegate Custom|leevent) (Utilities|Array|Get(acopy) (Variables|Default|GetTimerValues) (Variables|Default|GetCurrentBoost)) true))

(event Custom|UpdaterOfProfit
  ;[0.15 0.15 0.15 0.5] ProfitFromLevel
  (EventDispatchers|BindEventtoUpdateTimerLargeBattery (delegate Custom|StartTimer))
  (Utilities|Time|SetTimerbyEvent (delegate Custom|leevent) (Utilities|Array|Get(acopy) (Variables|Default|GetTimerValues) (Variables|Default|GetCurrentBoost)) true))

(event Custom|ChangeVolume
  ;[0.15 0.1473 0 0.5] MAIN
  ;;[0.15 0.15 0.15 0.5] SoundConstructions
  (Audio|Components|Audio|SetVolumeMultiplier (Variables|Default|GetSW_BigBatteryFinishedProduction) (Variables|/Game/Charapters/BP_Camera.BP_Camera_C|GetSoundMachineVolume (Variables|Default|GetBP_Camera)) :!class /Script/Engine.AudioComponent))

(event Custom|ChangeEffectVisibility
  (bind _bp_camera (Variables|Default|GetBP_Camera))
  (bind _staticmeshcomponent (Variables|Debug|GetStaticMeshComponent))
  (bind _effect (Variables|/Game/Charapters/BP_Camera.BP_Camera_C|GetEffect _bp_camera))
  ;[0.15 0.15 0.15 0.5] Effects
  (Development|SetHiddeninGame (Variables|Default|GetNFire_00) _effect false)
  (if _effect
    (Rendering|Material|SetOverlayMaterial _staticmeshcomponent 0 :!class /Script/Engine.MeshComponent)
    (else
      (Rendering|Material|SetOverlayMaterial _staticmeshcomponent "/Game/Project/MaterialLibrary/Materials/M_Outline.M_Outline" :!class /Script/Engine.MeshComponent))))

(event Custom|Effects
  ;[0.15 0.15 0.15 0.5] Effects
  (EventDispatchers|BindEventtoEDEffects (Variables|Default|GetBP_Camera) (delegate Custom|ChangeEffectVisibility)))

(event Custom|UpdateCostGainForSell
  (bind _level (Variables|Default|GetLevel))
  (bind _costofupdate (Variables|Default|GetCostOfUpdate))
  (bind _output (Utilities|Array|Get(acopy) _costofupdate _level))
  ;[0.15 0.15 0.15 0.5] CostGainForSell
  (switch int (Variables|Default|GetLevel)
    (:0
      (Variables|Default|SetCostForSellSilver (+ (Variables|Default|GetCostForSellSilver) _output)))
    (:1
      (Variables|Default|SetCostForSellGold (+ (Variables|Default|GetCostForSellGold) _output) :!label _label))
    (:2
      (goto _label))
    (:3
      (goto _label))
    (:4
      (goto _label))
    (:5
      (goto _label))))

(event Custom|Upgrader
  ;[0.15 0.1473 0 0.5] MAIN
  ;;[0.15 0.15 0.15 0.5] Events
  (Utilities|Time|SetTimerbyEvent (delegate Custom|Updatetimer) 0.1 true))

(event Custom|GetActorsOfClass
  ;[0.15 0.1473 0 0.5] MAIN
  ;;[0.15 0.15 0.15 0.5] GetActorsOfClass
  (bind _returnvalue (Actor|GetActorOfClass "/Game/Charapters/BP_Camera.BP_Camera_C"))
  (Variables|Default|SetBP_Camera _returnvalue))

(event Custom|UpdateMenuBeginPlay
  ;[0.15 0.15 0.15 0.5] UpdateMenu
  (EventDispatchers|BindEventtoRightClick (Variables|Default|GetBP_Camera) (delegate Custom|UpdateMenu)))

(event Custom|ChangeUpdateMenuCoin
  (bind _wbp_uiingame (Variables|Default|GetWBP_UIInGame))
  ;[0.15 0.15 0.15 0.5] ChangeUpdateMenuCoin
  (switch int (Variables|Default|GetLevel)
    (:0
      (Default|ChangeUpdateMenuCoin _wbp_uiingame 1))
    (:1
      (Default|ChangeUpdateMenuCoin _wbp_uiingame 2 :!label _label))
    (:2
      (goto _label))
    (:3
      (goto _label))
    (:4
      (goto _label))
    (:5
      (goto _label))))

(event Custom|ChangeDescriptionOfUpdateMenu
  ;[0.15 0.15 0.15 0.5] DescriptionOfUpdateMenu
  (Variables|/Script/UMG.TextBlock|SetText (Variables|/Game/Project/Blueprints/UI/Widgets/WBP_UIINGame.WBP_UIINGame_C|GetTXT_UpdateMenuChanges (Variables|Default|GetWBP_UIInGame)) (Utilities|Array|Get(acopy) (Variables|Default|GetWhatChangesByUpdate) (Variables|Default|GetLevel))))

(event Custom|CoinBackSystemBySell
  ;[0.15 0.15 0.15 0.5] CoinBackSustemBySell
  (if (Variables|/Game/Project/Blueprints/UI/Widgets/WBP_UIINGame.WBP_UIINGame_C|GetSellClicked (Variables|Default|GetWBP_UIInGame))
    (CallFunction|CoinBackSystem)
    (CallFunction|Sounds true false)
    (Default|CallDestroyed)
    (Actor|DestroyActor)))

(event Custom|IfTUpdateMenuBorderHidden,%20UpdateTarget%20=%20False
  ;[0.15 0.15 0.15 0.5] IfTUpdateMenuBorderHidden, UpdateTarget = False
  (switch Utilities|FlowControl|Switch|SwitchonESlateVisibility (Variables|/Script/UMG.Widget|GetVisibility (Variables|/Game/Project/Blueprints/UI/Widgets/WBP_UIINGame.WBP_UIINGame_C|GetT_UpdateMenuANDQuestMenuBorder (Variables|Default|GetWBP_UIInGame)))
    (:Hidden
      (Variables|Default|SetUpdateTarget false))))

(event EventBeginPlay
  ;[0.15 0.1473 0 0.5] MAIN
  ;;[0.15 0.15 0.15 0.5] EventBeginPlay
  (CallFunction|Upgrader)
  (CallFunction|GetActorsOfClass)
  (CallFunction|UpdateMenuBeginPlay)
  (CallFunction|UpdaterOfProfit)
  (CallFunction|SoundConstructions)
  (CallFunction|Effects))

(fn ConstructionScript)

(fn CoinBackSystem
  (bind _wbp_uiingame (Variables|Default|GetWBP_UIInGame))
  (bind _bp_camera (Variables|Default|GetBP_Camera))
  (bind _wbp_uiingame_2 (Variables|Default|GetWBP_UIInGame))
  (Variables|/Game/Charapters/BP_Camera.BP_Camera_C|SetBronze_Coin _bp_camera (+ (Variables|/Game/Charapters/BP_Camera.BP_Camera_C|GetBronze_Coin _bp_camera) (Variables|Default|GetCostForSellBronze)))
  (Variables|/Game/Charapters/BP_Camera.BP_Camera_C|SetSilver_Coin _bp_camera (+ (Variables|/Game/Charapters/BP_Camera.BP_Camera_C|GetSilver_Coin _bp_camera) (Variables|Default|GetCostForSellSilver) (Utilities|Array|Get(acopy) (Variables|/Game/Project/Blueprints/UI/Widgets/WBP_UIINGame.WBP_UIINGame_C|GetCostLargeBattery _wbp_uiingame_2) (Variables|/Game/Project/Blueprints/UI/Widgets/WBP_UIINGame.WBP_UIINGame_C|GetNumberOfCostLargeBattery _wbp_uiingame_2))))
  (Variables|/Game/Charapters/BP_Camera.BP_Camera_C|SetGold_Coin _bp_camera (+ (Variables|/Game/Charapters/BP_Camera.BP_Camera_C|GetGold_Coin _bp_camera) (Variables|Default|GetCostForSellGold)))
  (Widget|SetVisibility (Variables|/Game/Project/Blueprints/UI/Widgets/WBP_UIINGame.WBP_UIINGame_C|GetTextUpdateMenu _wbp_uiingame) "Hidden")
  (Widget|SetVisibility (Variables|/Game/Project/Blueprints/UI/Widgets/WBP_UIINGame.WBP_UIINGame_C|GetButtonUpdateMenu _wbp_uiingame) "Hidden")
  (Widget|SetVisibility (Variables|/Game/Project/Blueprints/UI/Widgets/WBP_UIINGame.WBP_UIINGame_C|GetTexuresUpdateMenu _wbp_uiingame) "Hidden")
  (Variables|Default|SetUpdateTarget false))