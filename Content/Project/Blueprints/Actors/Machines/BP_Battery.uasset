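; Battery machine actor that earns bronze, silver or gold coins by level on a looping boost-dependent timer, with Niagara and sound feedback.
; Right-clicking the hovered battery opens the shared upgrade menu and marks it as target.
; A 0.1-second timer polls that menu to update text, buy upgrades that swap meshes at tier changes, or sell with a refund.
; BP_Camera handles currency, input events and effect and volume settings.
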(event OnBeginCursorOver(StaticMeshComponent)
  (params (TouchedComponent :type Primitive%20Component%20Object%20Reference))
  ;[0.15 0.15 0.15 0.5] OpenUIUpdateMenu
  (Variables|Default|SetOnComponent true)
  (Rendering|Material|SetOverlayMaterial (Variables|Debug|GetStaticMeshComponent) "/Game/Project/MaterialLibrary/Materials/M_Outline.M_Outline" :!class /Script/Engine.MeshComponent))

(event OnEndCursorOver(StaticMeshComponent)
  (params (TouchedComponent :type Primitive%20Component%20Object%20Reference))
  ;[0.15 0.15 0.15 0.5] OpenUIUpdateMenu
  (Variables|Default|SetOnComponent false)
  (Rendering|Material|SetOverlayMaterial (Variables|Debug|GetStaticMeshComponent) 0 :!class /Script/Engine.MeshComponent))

(event OnClicked(StaticMeshComponent)
  (params (TouchedComponent :type Primitive%20Component%20Object%20Reference) (ButtonPressed :type Key%20Structure :default "None"))
  ;[0.15 0.15 0.15 0.5] Effects
  (Utilities|ClickAnimation))

(event Custom|UpdateMenu
  (bind _wbp_uiingame (Variables|Default|GetWBP_UIInGame))
  ;[0.15 0.15 0.15 0.5] OpenUIUpdateMenu
  (if (Variables|Default|GetOnComponent)
    (Variables|Default|SetUpdateTarget true)
    (Utilities|FlowControl|Sequence
      (:then_0
        (if (not (Variables|/Game/Project/Blueprints/UI/Widgets/WBP_UIINGame.WBP_UIINGame_C|GetRunBuildSelector _wbp_uiingame))
          (Widget|SetVisibility (Variables|/Game/Project/Blueprints/UI/Widgets/WBP_UIINGame.WBP_UIINGame_C|GetTextUpdateMenu _wbp_uiingame) "Visible")
          (Widget|SetVisibility (Variables|/Game/Project/Blueprints/UI/Widgets/WBP_UIINGame.WBP_UIINGame_C|GetButtonUpdateMenu _wbp_uiingame) "Visible")
          (Widget|SetVisibility (Variables|/Game/Project/Blueprints/UI/Widgets/WBP_UIINGame.WBP_UIINGame_C|GetTexuresUpdateMenu _wbp_uiingame) "Visible")))
      (:then_1
        (Utilities|ClickAnimation)))))

(event Custom|UpdateTimer
  ;[0.15 0.15 0.15 0.5] ProfitFromLevel
  (Utilities|Time|SetTimerbyEvent (delegate Custom|leevent) (Utilities|Array|Get(acopy) (Variables|Default|GetTimerValues) (Variables|Default|GetCurrentBoost)) true))

(event Custom|leevent
  (bind _bp_camera (Variables|Default|GetBP_Camera))
  (bind _effect (Variables|/Game/Charapters/BP_Camera.BP_Camera_C|GetEffect _bp_camera))
  ;[0.15 0.15 0.15 0.5] ProfitFromLevel
  (switch int (Variables|Default|GetLevel)
    (:0
      (Variables|Default|SetCoinTypeForAdd 0 :!label _label)
      (Utilities|Effect (Variables|Default|GetNS_BronzeCoin) _effect
        (:Output
          (Default|ChangeCoins (Variables|Default|GetBP_Camera) (Variables|Default|GetCoinTypeForSubtract) (Variables|Default|GetLevel) 0 false (Variables|Default|GetProfit) (Variables|Default|GetCoinTypeForAdd) :!label _label_2)
          (CallFunction|Sounds false false))))
    (:1
      (goto _label))
    (:2
      (goto _label))
    (:3
      (goto _label))
    (:4
      (Variables|Default|SetCoinTypeForAdd 1 :!label _label_3)
      (Utilities|Effect (Variables|Default|GetNS_BronzeCoin2) _effect
        (:Output
          (goto _label_2))))
    (:5
      (goto _label_3))
    (:6
      (goto _label_3))
    (:7
      (goto _label_3))
    (:8
      (goto _label_3))
    (:9
      (Variables|Default|SetCoinTypeForAdd 2 :!label _label_4)
      (Utilities|Effect (Variables|Default|GetNS_GoldCoin) _effect
        (:Output
          (Utilities|FlowControl|Sequence
            (:then_0
              (goto _label_2))
            (:then_1
              (Utilities|FlowControl|DoOnce false
                (:Completed
                  (Transformation|AddLocalOffset (Variables|Default|GetNS_GoldCoin) "0.000000,0.000000,125.000000" false false))))))))
    (:10
      (goto _label_4))))

(event Custom|UpdateTextCost
  (bind _level (Variables|Default|GetLevel))
  (bind _wbp_uiingame (Variables|Default|GetWBP_UIInGame))
  (bind _txt_costofupdate (Variables|/Game/Project/Blueprints/UI/Widgets/WBP_UIINGame.WBP_UIINGame_C|GetTXT_CostOfUpdate _wbp_uiingame))
  ;[0.15 0.15 0.15 0.5] UpdateTextCost
  (if (== _level 10)
    (Rendering|Components|TextRender|SetText _txt_costofupdate "MAX")
    (else
      (Rendering|Components|TextRender|SetText _txt_costofupdate (Utilities|Text|ToText(Integer) (Utilities|Array|Get(acopy) (Variables|Default|GetCostOfUpdate) _level))))))

(event Custom|Upgrade
  ;[0.15 0.15 0.15 0.5] Upgrade
  (if (Variables|/Game/Project/Blueprints/UI/Widgets/WBP_UIINGame.WBP_UIINGame_C|GetUpdateCliked (Variables|Default|GetWBP_UIInGame))
    (if (< (Variables|Default|GetLevel) 10)
      (switch int (Variables|Default|GetLevel)
        (:0
          (Variables|Default|SetCoinTypeForSubtract 0 :!label _label))
        (:1
          (goto _label))
        (:2
          (goto _label))
        (:3
          (goto _label))
        (:4
          (goto _label))
        (:5
          (Variables|Default|SetCoinTypeForSubtract 1 :!label _label_2))
        (:6
          (goto _label_2))
        (:7
          (goto _label_2))
        (:8
          (goto _label_2))
        (:9
          (goto _label_2))
        (:10
          (Variables|Default|SetCoinTypeForSubtract 2)))
      (bind _done (Default|ChangeCoins (Variables|Default|GetBP_Camera) (Variables|Default|GetCoinTypeForSubtract) (Variables|Default|GetLevel) (Variables|Default|GetCostOfUpdate) true))
      (if _done
        (Variables|/Game/Project/Blueprints/UI/Widgets/WBP_UIINGame.WBP_UIINGame_C|SetUpdateCliked (Variables|Default|GetWBP_UIInGame) false)
        (CallFunction|UpdateCostGainforSell)
        (CallFunction|Sounds false true)
        (Variables|Default|SetLevel (+ (Variables|Default|GetLevel) 1))
        ;[0.15 0.15 0.15 0.5] StaticMesh
        (switch int (Variables|Default|GetLevel)
          (:4
            (Components|StaticMesh|SetStaticMesh (Variables|Debug|GetStaticMeshComponent) "/Game/Project/MaterialLibrary/Meshes/engine_2nd_lvl.engine_2nd_lvl")
            (Transformation|AddActorWorldOffset "0.000000,0.000000,350.000000"))
          (:9
            (Components|StaticMesh|SetStaticMesh (Variables|Debug|GetStaticMeshComponent) "/Game/Project/MaterialLibrary/Meshes/engine_3rd_lvl.engine_3rd_lvl")))
        (else
          (Default|Sounds (Variables|Default|GetBP_Camera) false false false false false true))))))

(event Custom|Sounds
  (params (Selling :type Boolean) (Upgrade :type Boolean))
  ;[0.15 0.15 0.15 0.5] Sounds
  (if (or Selling Upgrade)
    (Default|Sounds (Variables|Default|GetBP_Camera) false false Selling false Upgrade false)
    (else
      (Audio|Components|Audio|Play (Variables|Default|GetSW_WorkingMachine) 0.0))))

(event Custom|SoundConstructions
  ;[0.15 0.1473 0 0.5] MAIN
  ;;[0.15 0.15 0.15 0.5] SoundConstructions
  (EventDispatchers|BindEventtoEDSoundMachineVolume (Variables|Default|GetBP_Camera) (delegate Custom|ChangeVolume))
  (Audio|Components|Audio|SetVolumeMultiplier (Variables|Default|GetSW_WorkingMachine) (Variables|Default|GetSoundMachineVolume) :!class /Script/Engine.AudioComponent))

(event Custom|ChangeVolume
  ;[0.15 0.1473 0 0.5] MAIN
  ;;[0.15 0.15 0.15 0.5] SoundConstructions
  (Audio|Components|Audio|SetVolumeMultiplier (Variables|Default|GetSW_WorkingMachine) (Variables|/Game/Charapters/BP_Camera.BP_Camera_C|GetSoundMachineVolume (Variables|Default|GetBP_Camera)) :!class /Script/Engine.AudioComponent))

(event Custom|ChangeEffectVisibility
  (bind _staticmeshcomponent (Variables|Debug|GetStaticMeshComponent))
  ;[0.15 0.15 0.15 0.5] Effects
  (if (Variables|/Game/Charapters/BP_Camera.BP_Camera_C|GetEffect (Variables|Default|GetBP_Camera))
    (Rendering|Material|SetOverlayMaterial _staticmeshcomponent 0 :!class /Script/Engine.MeshComponent)
    (else
      (Rendering|Material|SetOverlayMaterial _staticmeshcomponent "/Game/Project/MaterialLibrary/Materials/M_Outline.M_Outline" :!class /Script/Engine.MeshComponent))))

(event Custom|Effects
  ;[0.15 0.15 0.15 0.5] Effects
  (Components|Activation|Deactivate (Variables|Default|GetNS_BronzeCoin))
  (EventDispatchers|BindEventtoEDEffects (Variables|Default|GetBP_Camera) (delegate Custom|ChangeEffectVisibility)))

(event Custom|UpdateCostGainForSell
  (bind _level (Variables|Default|GetLevel))
  (bind _costofupdate (Variables|Default|GetCostOfUpdate))
  (bind _output (Utilities|Array|Get(acopy) _costofupdate _level))
  ;[0.15 0.15 0.15 0.5] CostGainForSell
  (switch int (Variables|Default|GetLevel)
    (:0
      (Variables|Default|SetCostForSellBronze (+ (Variables|Default|GetCostForSellBronze) _output) :!label _label))
    (:1
      (goto _label))
    (:2
      (goto _label))
    (:3
      (goto _label))
    (:4
      (goto _label))
    (:5
      (Variables|Default|SetCostForSellSilver (+ (Variables|Default|GetCostForSellSilver) _output) :!label _label_2))
    (:6
      (goto _label_2))
    (:7
      (goto _label_2))
    (:8
      (goto _label_2))
    (:9
      (goto _label_2))
    (:10
      (Variables|Default|SetCostForSellGold (+ (Variables|Default|GetCostForSellGold) _output)))))

(event Custom|UpdaterTimer
  ;[0.15 0.1473 0 0.5] MAIN
  ;;[0.15 0.15 0.15 0.5] Events
  (Utilities|FlowControl|Sequence
    (:then_0
      (if (Variables|Default|GetUpdateTarget)
        (CallFunction|ChangeUpdateMenuCoin)
        (CallFunction|ChangeDescriptionOfUpdateMenu)
        (CallFunction|CoinBackSystembySell)
        (CallFunction|UpdateTextCost)
        (CallFunction|Upgrade)))
    (:then_1
      (CallFunction|IfTUpdateMenuBorderHidden,UpdateTarget=False))))

(event Custom|UpdaterOfProfit
  ;[0.15 0.15 0.15 0.5] ProfitFromLevel
  (EventDispatchers|BindEventtoUpdatebatteryTimer (delegate Custom|UpdateTimer))
  (Utilities|Time|SetTimerbyEvent (delegate Custom|leevent) (Utilities|Array|Get(acopy) (Variables|Default|GetTimerValues) (Variables|Default|GetCurrentBoost)) true))

(event Custom|Upgrader
  ;[0.15 0.1473 0 0.5] MAIN
  ;;[0.15 0.15 0.15 0.5] Events
  (Utilities|Time|SetTimerbyEvent (delegate Custom|UpdaterTimer) 0.1 true))

(event Custom|GetActorsOfClass
  ;[0.15 0.1473 0 0.5] MAIN
  ;;[0.15 0.15 0.15 0.5] GetActorsOfClass
  (bind _returnvalue (Actor|GetActorOfClass "/Game/Charapters/BP_Camera.BP_Camera_C"))
  (Variables|Default|SetBP_Camera _returnvalue))

(event Custom|UpdateMenuBeginPlay
  ;[0.15 0.15 0.15 0.5] OpenUIUpdateMenu
  (EventDispatchers|BindEventtoRightClick (Variables|Default|GetBP_Camera) (delegate Custom|UpdateMenu)))

(event Custom|ChangeUpdateMenuCoin
  (bind _wbp_uiingame (Variables|Default|GetWBP_UIInGame))
  ;[0.15 0.15 0.15 0.5] ChangeUpdateMenuCoin
  (switch int (Variables|Default|GetLevel)
    (:0
      (Default|ChangeUpdateMenuCoin _wbp_uiingame :!label _label))
    (:1
      (goto _label))
    (:2
      (goto _label))
    (:3
      (goto _label))
    (:4
      (goto _label))
    (:5
      (Default|ChangeUpdateMenuCoin _wbp_uiingame 1 :!label _label_2))
    (:6
      (goto _label_2))
    (:7
      (goto _label_2))
    (:8
      (goto _label_2))
    (:9
      (goto _label_2))
    (:10
      (Default|ChangeUpdateMenuCoin _wbp_uiingame 2))))

(event Custom|ChangeDescriptionOfUpdateMenu
  ;[0.15 0.15 0.15 0.5] DescriptionOfUpdateMenu
  (Variables|/Script/UMG.TextBlock|SetText (Variables|/Game/Project/Blueprints/UI/Widgets/WBP_UIINGame.WBP_UIINGame_C|GetTXT_UpdateMenuChanges (Variables|Default|GetWBP_UIInGame)) (Utilities|Array|Get(acopy) (Variables|Default|GetWhatChangesByUpdate) (Variables|Default|GetLevel))))

(event Custom|CoinBackSystemBySell
  ;[0.15 0.15 0.15 0.5] CoinBackSustemBySell
  (if (Variables|/Game/Project/Blueprints/UI/Widgets/WBP_UIINGame.WBP_UIINGame_C|GetSellClicked (Variables|Default|GetWBP_UIInGame))
    (CallFunction|CoinBackSystem)
    (CallFunction|Sounds true false)
    (Default|CallDestroyed)
    (Actor|DestroyActor)))

(event Custom|IfTUpdateMenuBorderHidden,%20UpdateTarget%20=%20False
  ;[0.15 0.15 0.15 0.5] IfTUpdateMenuBorderHidden, UpdateTarget = False
  (switch Utilities|FlowControl|Switch|SwitchonESlateVisibility (Variables|/Script/UMG.Widget|GetVisibility (Variables|/Game/Project/Blueprints/UI/Widgets/WBP_UIINGame.WBP_UIINGame_C|GetT_UpdateMenuANDQuestMenuBorder (Variables|Default|GetWBP_UIInGame)))
    (:Hidden
      (Variables|Default|SetUpdateTarget false))))

(event EventBeginPlay
  ;[0.15 0.1473 0 0.5] MAIN
  ;;[0.15 0.15 0.15 0.5] EventBeginPlay
  (CallFunction|Upgrader)
  (CallFunction|GetActorsOfClass)
  (CallFunction|UpdateMenuBeginPlay)
  (CallFunction|UpdaterOfProfit)
  (CallFunction|SoundConstructions)
  (CallFunction|Effects))

(fn ConstructionScript)

(fn Produce
  (params (2x :type Boolean) (CurrentLevel :type Integer)))

(fn CoinBackSystem
  (bind _wbp_uiingame (Variables|Default|GetWBP_UIInGame))
  (bind _bp_camera (Variables|Default|GetBP_Camera))
  (bind _wbp_uiingame_2 (Variables|Default|GetWBP_UIInGame))
  (Variables|/Game/Charapters/BP_Camera.BP_Camera_C|SetBronze_Coin _bp_camera (+ (Variables|/Game/Charapters/BP_Camera.BP_Camera_C|GetBronze_Coin _bp_camera) (Variables|Default|GetCostForSellBronze) (Utilities|Array|Get(acopy) (Variables|/Game/Project/Blueprints/UI/Widgets/WBP_UIINGame.WBP_UIINGame_C|GetCostBattery _wbp_uiingame_2) (Variables|/Game/Project/Blueprints/UI/Widgets/WBP_UIINGame.WBP_UIINGame_C|GetNumberOfCostBattery _wbp_uiingame_2))))
  (Variables|/Game/Charapters/BP_Camera.BP_Camera_C|SetSilver_Coin _bp_camera (+ (Variables|/Game/Charapters/BP_Camera.BP_Camera_C|GetSilver_Coin _bp_camera) (Variables|Default|GetCostForSellSilver)))
  (Variables|/Game/Charapters/BP_Camera.BP_Camera_C|SetGold_Coin _bp_camera (+ (Variables|/Game/Charapters/BP_Camera.BP_Camera_C|GetGold_Coin _bp_camera) (Variables|Default|GetCostForSellGold)))
  (Widget|SetVisibility (Variables|/Game/Project/Blueprints/UI/Widgets/WBP_UIINGame.WBP_UIINGame_C|GetTextUpdateMenu _wbp_uiingame) "Hidden")
  (Widget|SetVisibility (Variables|/Game/Project/Blueprints/UI/Widgets/WBP_UIINGame.WBP_UIINGame_C|GetButtonUpdateMenu _wbp_uiingame) "Hidden")
  (Widget|SetVisibility (Variables|/Game/Project/Blueprints/UI/Widgets/WBP_UIINGame.WBP_UIINGame_C|GetTexuresUpdateMenu _wbp_uiingame) "Hidden")
  (Variables|Default|SetUpdateTarget false))