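; BP_AirSheap is a purchasable, clickable airship actor that ends the game with a win when launched.
; It binds to the in-game widget's purchase event via BP_Camera and, once purchased, unhides itself and its text label.
; Clicking it while visible hides the label, adds audio and starts a looping timer that moves it along X.
; After a delay it shows WBP_Win in place of all widgets, then opens L_Base.
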(event OnClicked(StaticMeshComponent)
  (params (TouchedComponent :type Primitive%20Component%20Object%20Reference) (ButtonPressed :type Key%20Structure :default "None"))
  (if (not (Variables|Rendering|GetbHidden))
    (Development|SetHiddeninGame (Variables|Default|GetTextRender) true false)
    (Utilities|Time|SetTimerbyEvent (delegate Custom|FlyAway) 0.05 true)
    (AddComponent|AddAudioComponent false)
    (Utilities|FlowControl|Delay 5.0)
    (Viewport|RemoveAllWidgets)
    (bind _returnvalue (Game|ConstructObjectfromClass "/Game/Project/Blueprints/UI/Widgets/WBP_Win.WBP_Win_C"))
    (UserInterface|Viewport|AddtoViewport _returnvalue 0)
    (Utilities|FlowControl|Delay 2.0)
    (Game|OpenLevel(byObjectReference) "/Game/Project/Levels/L_Base.L_Base")))

(event Custom|FlyAway
  (Transformation|AddActorWorldOffset (Math|Vector|MakeVector (Math|Conversions|ToFloat(Integer) (- (Variables|Default|GetFlyyyyy) 100)) 0.0 0.0)))

(event Custom|AirSheapPurchased
  (Utilities|FlowControl|DoOnce false
    (:Completed
      (Rendering|SetActorHiddenInGame false)
      (Development|SetHiddeninGame (Variables|Default|GetTextRender) false false))))

(event EventBeginPlay
  (bind _returnvalue (Actor|GetActorOfClass "/Game/Charapters/BP_Camera.BP_Camera_C"))
  (bind _output_get (Variables|Default|SetBP_Camera _returnvalue))
  (Utilities|FlowControl|Delay 0.2)
  (EventDispatchers|BindEventtoPurchasedAirSheap (Variables|/Game/Charapters/BP_Camera.BP_Camera_C|GetWBP_UIInGame _output_get) (delegate Custom|AirSheapPurchased)))

(fn ConstructionScript)