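; BP_Platform is a buyable land tile that machines are built on, priced in bronze, silver or gold coins by ID.
; In shop mode it shows a hoverable placeholder and timer-refreshed price from the in-game widget.
; Buying spends BP_Camera coins, raises the shared price level and reveals the randomly textured platform and grid, unless open from start.
; Its spawned BP_ForMachine receives hover state and is flagged built on a build-mode click.
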(event OnBeginCursorOver(PrePlatform)
  (params (TouchedComponent :type Primitive%20Component%20Object%20Reference))
  ;[0.15 0.15 0.15 0.5] PlatformSelect
  (if (Variables|/Game/Project/Blueprints/UI/Widgets/WBP_UIINGame.WBP_UIINGame_C|GetInShop (Variables|Default|GetWbpuiInGAmE))
    (Rendering|Material|SetMaterial TouchedComponent 0 "/Game/Project/MaterialLibrary/Materials/M_CursorOnPlatform.M_CursorOnPlatform")))

(event OnBeginCursorOver(Platform)
  (params (TouchedComponent :type Primitive%20Component%20Object%20Reference))
  ;[0.15 0.15 0.15 0.5] SpawnForMachineMouseWork
  (Variables|/Game/Project/Blueprints/Actors/Machines/BP_ForMachine.BP_ForMachine_C|SetCursorOnPlatform (Variables|Default|GetSpawnedForMachine) true))

(event OnEndCursorOver(Platform)
  (params (TouchedComponent :type Primitive%20Component%20Object%20Reference))
  ;[0.15 0.15 0.15 0.5] SpawnForMachineMouseWork
  (Variables|/Game/Project/Blueprints/Actors/Machines/BP_ForMachine.BP_ForMachine_C|SetCursorOnPlatform (Variables|Default|GetSpawnedForMachine) false))

(event OnEndCursorOver(PrePlatform)
  (params (TouchedComponent :type Primitive%20Component%20Object%20Reference))
  ;[0.15 0.15 0.15 0.5] PlatformSelect
  (if (Variables|/Game/Project/Blueprints/UI/Widgets/WBP_UIINGame.WBP_UIINGame_C|GetInShop (Variables|Default|GetWbpuiInGAmE))
    (Rendering|Material|SetMaterial TouchedComponent 0 "/Game/Project/MaterialLibrary/Materials/M_PrePlatformTest.M_PrePlatformTest")))

(event OnClicked(PrePlatform)
  (params (TouchedComponent :type Primitive%20Component%20Object%20Reference) (ButtonPressed :type Key%20Structure :default "None"))
  (bind _wbpuiingame (Variables|Default|GetWbpuiInGAmE))
  (bind _preplatform (Variables|Default|GetPrePlatform))
  (bind _id (Variables|Default|GetID))
  (bind _wbpuiingame_2 (Variables|Default|GetWbpuiInGAmE))
  (bind _wbpuiingame_3 (Variables|Default|GetWbpuiInGAmE))
  ;[0.15 0.15 0.15 0.5] OpenTerritory
  (switch int (Variables|Default|GetID)
    (:0
      (Utilities|Uhh :!label _label
        (:>=Bronze
          _)
        (:>=Silver
          _)
        (:>=Gold
          _))
      (Rendering|SetVisibility _preplatform false false)
      (Components|MoveComponentTo _preplatform "0.000000,0.000000,-1000000.000000" "0, 0, 0" false false 0.2 false)
      (Rendering|SetVisibility (Variables|Default|GetPlatform) true false)
      (Variables|Default|SetOpenSetka true)
      (CallFunction|SetVisibleSetkabyBuying true)
      (if (not (Variables|Default|GetOpenInStart))
        (switch int _id
          (:0
            (Default|ChangeCoins (Variables|Default|GetBP_Camera) _id (Variables|/Game/Project/Blueprints/UI/Widgets/WBP_UIINGame.WBP_UIINGame_C|GetLevelOfPlatformPriceBronze _wbpuiingame_2) (Variables|/Game/Project/Blueprints/UI/Widgets/WBP_UIINGame.WBP_UIINGame_C|GetPlatformPriceBronze _wbpuiingame_2) true)
            (Math|Integer|IncrementInt (Variables|/Game/Project/Blueprints/UI/Widgets/WBP_UIINGame.WBP_UIINGame_C|GetLevelOfPlatformPriceBronze (Variables|Default|GetWbpuiInGAmE))))
          (:1
            (Default|ChangeCoins (Variables|Default|GetBP_Camera) _id (Variables|/Game/Project/Blueprints/UI/Widgets/WBP_UIINGame.WBP_UIINGame_C|GetLevelOfPlatformPriceSilver _wbpuiingame_3) (Variables|/Game/Project/Blueprints/UI/Widgets/WBP_UIINGame.WBP_UIINGame_C|GetPlatformPriceSilver _wbpuiingame_3) true)
            (Math|Integer|IncrementInt (Variables|/Game/Project/Blueprints/UI/Widgets/WBP_UIINGame.WBP_UIINGame_C|GetLevelOfPlatformPriceSilver (Variables|Default|GetWbpuiInGAmE))))
          (:2
            (Default|ChangeCoins (Variables|Default|GetBP_Camera) _id (Variables|/Game/Project/Blueprints/UI/Widgets/WBP_UIINGame.WBP_UIINGame_C|GetLevelOfPlatformPriceGold _wbpuiingame) (Variables|/Game/Project/Blueprints/UI/Widgets/WBP_UIINGame.WBP_UIINGame_C|GetPlatformPriceGold _wbpuiingame) true)
            (Math|Integer|IncrementInt (Variables|/Game/Project/Blueprints/UI/Widgets/WBP_UIINGame.WBP_UIINGame_C|GetLevelOfPlatformPriceGold (Variables|Default|GetWbpuiInGAmE)))))))
    (:1
      (goto _label Silver))
    (:2
      (goto _label Gold))))

(event OnClicked(Platform)
  (params (TouchedComponent :type Primitive%20Component%20Object%20Reference) (ButtonPressed :type Key%20Structure :default "None"))
  (bind _wbpuiingame (Variables|Default|GetWbpuiInGAmE))
  ;[0.15 0.15 0.15 0.5] SpawnForMachineMouseWork
  (if (and (Variables|/Game/Project/Blueprints/UI/Widgets/WBP_UIINGame.WBP_UIINGame_C|GetRunBuildSelector _wbpuiingame) (not (Variables|/Game/Project/Blueprints/Actors/Machines/BP_ForMachine.BP_ForMachine_C|GetStop (Variables|Default|GetSpawnedForMachine))))
    (Variables|/Game/Project/Blueprints/Actors/Machines/BP_ForMachine.BP_ForMachine_C|SetBuilded (Variables|Default|GetSpawnedForMachine) true)
    (Variables|Default|SetBuildedZone true)
    (Variables|/Game/Project/Blueprints/UI/Widgets/WBP_UIINGame.WBP_UIINGame_C|SetRunBuildSelector _wbpuiingame false)))

(event Custom|ChangeSprite
  (bind _t_bronzecoin2_sprite (Variables|Default|GetT_BronzeCoin2_Sprite))
  ;[0.15 0.15 0.15 0.5] ChangeSprite
  (switch int (Variables|Default|GetID)
    (:0
      (Rendering|Components|Sprite|SetSprite _t_bronzecoin2_sprite "/Game/Project/MaterialLibrary/Textures/T_BronzeCoin2_Sprite.T_BronzeCoin2_Sprite"))
    (:1
      (Rendering|Components|Sprite|SetSprite _t_bronzecoin2_sprite "/Game/Project/MaterialLibrary/Textures/T_SilverCoin2_Sprite.T_SilverCoin2_Sprite"))
    (:2
      (Rendering|Components|Sprite|SetSprite _t_bronzecoin2_sprite "/Game/Project/MaterialLibrary/Textures/T_GoldCoin2_Sprite.T_GoldCoin2_Sprite"))))

(event Custom|OpenZone
  (bind _wbpuiingame (Variables|Default|GetWbpuiInGAmE))
  (bind _preplatform (Variables|Default|GetPrePlatform))
  (bind _id (Variables|Default|GetID))
  (bind _wbpuiingame_2 (Variables|Default|GetWbpuiInGAmE))
  (bind _wbpuiingame_3 (Variables|Default|GetWbpuiInGAmE))
  ;[0.15 0.15 0.15 0.5] OpenTerritory
  (if (not (Variables|Default|GetOpenInStart))
    ;[0.15 0.15 0.15 0.5] ChangeTextOfPlatformPrice
    (Utilities|Time|SetTimerbyEvent (delegate Custom|CustomEvent) 0.1 true)
    (else
      (Rendering|SetVisibility _preplatform false false)
      (Components|MoveComponentTo _preplatform "0.000000,0.000000,-1000000.000000" "0, 0, 0" false false 0.2 false)
      (Rendering|SetVisibility (Variables|Default|GetPlatform) true false)
      (Variables|Default|SetOpenSetka true)
      (CallFunction|SetVisibleSetkabyBuying true)
      (if (not (Variables|Default|GetOpenInStart))
        (switch int _id
          (:0
            (Default|ChangeCoins (Variables|Default|GetBP_Camera) _id (Variables|/Game/Project/Blueprints/UI/Widgets/WBP_UIINGame.WBP_UIINGame_C|GetLevelOfPlatformPriceBronze _wbpuiingame_2) (Variables|/Game/Project/Blueprints/UI/Widgets/WBP_UIINGame.WBP_UIINGame_C|GetPlatformPriceBronze _wbpuiingame_2) true)
            (Math|Integer|IncrementInt (Variables|/Game/Project/Blueprints/UI/Widgets/WBP_UIINGame.WBP_UIINGame_C|GetLevelOfPlatformPriceBronze (Variables|Default|GetWbpuiInGAmE))))
          (:1
            (Default|ChangeCoins (Variables|Default|GetBP_Camera) _id (Variables|/Game/Project/Blueprints/UI/Widgets/WBP_UIINGame.WBP_UIINGame_C|GetLevelOfPlatformPriceSilver _wbpuiingame_3) (Variables|/Game/Project/Blueprints/UI/Widgets/WBP_UIINGame.WBP_UIINGame_C|GetPlatformPriceSilver _wbpuiingame_3) true)
            (Math|Integer|IncrementInt (Variables|/Game/Project/Blueprints/UI/Widgets/WBP_UIINGame.WBP_UIINGame_C|GetLevelOfPlatformPriceSilver (Variables|Default|GetWbpuiInGAmE))))
          (:2
            (Default|ChangeCoins (Variables|Default|GetBP_Camera) _id (Variables|/Game/Project/Blueprints/UI/Widgets/WBP_UIINGame.WBP_UIINGame_C|GetLevelOfPlatformPriceGold _wbpuiingame) (Variables|/Game/Project/Blueprints/UI/Widgets/WBP_UIINGame.WBP_UIINGame_C|GetPlatformPriceGold _wbpuiingame) true)
            (Math|Integer|IncrementInt (Variables|/Game/Project/Blueprints/UI/Widgets/WBP_UIINGame.WBP_UIINGame_C|GetLevelOfPlatformPriceGold (Variables|Default|GetWbpuiInGAmE)))))))))

(event Custom|SetVisibleSetkaByBuying
  (params (SetkaBuy :type Boolean))
  ;[0.15 0.15 0.15 0.5] Buy Zones
  (CallFunction|SetPlatformANDSetkaVisibility (Variables|/Game/Project/Blueprints/UI/Widgets/WBP_UIINGame.WBP_UIINGame_C|GetInShop (Variables|Default|GetWbpuiInGAmE)) SetkaBuy))

(event Custom|CustomEvent
  (bind _wbpuiingame (Variables|Default|GetWbpuiInGAmE))
  (bind _wbpuiingame_2 (Variables|Default|GetWbpuiInGAmE))
  (bind _wbpuiingame_3 (Variables|Default|GetWbpuiInGAmE))
  (bind _platformpricebronze (Variables|/Game/Project/Blueprints/UI/Widgets/WBP_UIINGame.WBP_UIINGame_C|GetPlatformPriceBronze _wbpuiingame_2))
  (bind _levelofplatformpricebronze (Variables|/Game/Project/Blueprints/UI/Widgets/WBP_UIINGame.WBP_UIINGame_C|GetLevelOfPlatformPriceBronze _wbpuiingame_2))
  (bind _platformpricesilver (Variables|/Game/Project/Blueprints/UI/Widgets/WBP_UIINGame.WBP_UIINGame_C|GetPlatformPriceSilver _wbpuiingame_3))
  (bind _levelofplatformpricesilver (Variables|/Game/Project/Blueprints/UI/Widgets/WBP_UIINGame.WBP_UIINGame_C|GetLevelOfPlatformPriceSilver _wbpuiingame_3))
  (bind _platformpricegold (Variables|/Game/Project/Blueprints/UI/Widgets/WBP_UIINGame.WBP_UIINGame_C|GetPlatformPriceGold _wbpuiingame))
  (bind _levelofplatformpricegold (Variables|/Game/Project/Blueprints/UI/Widgets/WBP_UIINGame.WBP_UIINGame_C|GetLevelOfPlatformPriceGold _wbpuiingame))
  (bind _output (Utilities|Array|Get(acopy) _platformpricegold _levelofplatformpricegold))
  (bind _output_2 (Utilities|Array|Get(acopy) _platformpricebronze _levelofplatformpricebronze))
  (bind _output_3 (Utilities|Array|Get(acopy) _platformpricesilver _levelofplatformpricesilver))
  ;[0.15 0.15 0.15 0.5] ChangeTextOfPlatformPrice
  (if (not (Variables|Default|GetOpenSetka))
    (switch int (Variables|Default|GetID)
      (:0
        (if (not (== (Variables|Default|GetPriceOldBronze) _output_2))
          (Variables|Default|SetPriceOldBronze 0)
          (Rendering|Components|TextRender|SetText (Variables|Default|GetTextRender) (Utilities|Text|ToText(Integer) _output_2))))
      (:1
        (if (not (== (Variables|Default|GetPriceOldSilver) _output_3))
          (Variables|Default|SetPriceOldSilver 0)
          (Rendering|Components|TextRender|SetText (Variables|Default|GetTextRender) (Utilities|Text|ToText(Integer) _output_3))))
      (:2
        (if (not (== (Variables|Default|GetPriceOldGold) _output))
          (Variables|Default|SetPriceOldGold 0)
          (Rendering|Components|TextRender|SetText (Variables|Default|GetTextRender) (Utilities|Text|ToText(Integer) _output)))))))

(event Custom|SetMaterial
  (bind _platform (Variables|Default|GetPlatform))
  ;[0.15 0.15 0.15 0.5] MaterialPlatform
  (switch int (Math|Random|RandomIntegerinRange 0 1)
    (:0
      (Rendering|Material|SetMaterial _platform 0 "/Game/Project/MaterialLibrary/Materials/M_PlatformType1.M_PlatformType1"))
    (:1
      (Rendering|Material|SetMaterial _platform 0 "/Game/Project/MaterialLibrary/Materials/M_PlatformType2.M_PlatformType2"))))

(event Custom|GetActorsOfClass
  ;[0.15 0.1473 0 0.5] MAIN
  ;;[0.15 0.15 0.15 0.5] GetActorsOfClass
  (bind _returnvalue (Actor|GetActorOfClass "/Game/Charapters/BP_Camera.BP_Camera_C"))
  (Variables|Default|SetBP_Camera _returnvalue))

(event Custom|Events
  ;[0.15 0.1473 0 0.5] MAIN
  ;;[0.15 0.15 0.15 0.5] Events
  (CallFunction|SetMaterial)
  (CallFunction|BuyZonesSystem)
  (CallFunction|SpawnBPforMachine)
  (CallFunction|OpenZone)
  (CallFunction|ChangeSprite))

(event Custom|PlayerInShop
  ;[0.15 0.15 0.15 0.5] Buy Zones
  (CallFunction|SetPlatformANDSetkaVisibility (Variables|/Game/Project/Blueprints/UI/Widgets/WBP_UIINGame.WBP_UIINGame_C|GetInShop (Variables|Default|GetWbpuiInGAmE)) (stale Custom|SetVisibleSetkaByBuying SetkaBuy)))

(event Custom|BuyZonesSystem
  ;[0.15 0.15 0.15 0.5] Buy Zones
  (Utilities|FlowControl|Delay 0.1)
  (EventDispatchers|BindEventtoEDinShop (Variables|Default|GetWbpuiInGAmE) (delegate Custom|PlayerInShop)))

(event Custom|SpawnBP_ForMachine
  ;[0.15 0.15 0.15 0.5] Spawn BP_ForMachine
  (bind _returnvalue (Game|SpawnActorfromClass "/Game/Project/Blueprints/Actors/Machines/BP_ForMachine.BP_ForMachine_C" (Transformation|GetActorTransform) "Undefined" "MultiplyWithRoot" 0 0))
  (Variables|Default|SetSpawnedForMachine _returnvalue))

(event EventBeginPlay
  ;[0.15 0.1473 0 0.5] MAIN
  ;;[0.15 0.15 0.15 0.5] EventBeginPlay
  (CallFunction|GetActorsOfClass)
  (CallFunction|Events))

(fn ConstructionScript)

(fn SetPlatformANDSetkaVisibility
  (params (Visibility :type Boolean) (SetkaBuy :type Boolean))
  (Utilities|FlowControl|Sequence
    (:then_0
      (Rendering|SetVisibility (Variables|Default|GetTextRender) Visibility false)
      (Rendering|SetVisibility (Variables|Default|GetPrePlatform) Visibility false)
      (Rendering|SetVisibility (Variables|Default|GetT_BronzeCoin2_Sprite) Visibility false)
      (if (Variables|Default|GetOpenSetka)
        (Rendering|SetVisibility (Variables|Default|GetSetka) Visibility false)))
    (:then_1
      (if SetkaBuy
        (Rendering|SetVisibility (Variables|Default|GetSetka) true false)
        (CallFunction|SetVisibleSetkabyBuying false)))))