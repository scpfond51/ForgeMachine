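; BP_Cloud is a local fog volume cloud that, unless flagged Static, drifts along world X and destroys itself after a fixed number of steps.
; On BeginPlay, non-static clouds start a looping movement timer and randomly pick one of three grey shades, with the two darker ones placed progressively lower.
; They also bind to BP_Camera's effects dispatcher, which toggles fog visibility from effect flags.
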(event Custom|FogMovement
  (Transformation|AddActorWorldOffset "300.000000,0.000000,0.000000")
  (bind _result (Math|Integer|IncrementInt (Variables|Default|GetLocation))
    (:%20%20
      (if (== _result 900)
        (Actor|DestroyActor)))))

(event Custom|Effects
  (Development|SetHiddeninGame (Variables|Default|GetLocalFogVolume) (or (Variables|/Game/Charapters/BP_Camera.BP_Camera_C|GetEffect (Variables|Default|GetBP_Camera)) (Variables|Default|GetEffect)) false))

(event EventBeginPlay
  (bind _returnvalue (Actor|GetActorOfClass "/Game/Charapters/BP_Camera.BP_Camera_C"))
  (Variables|Default|SetBP_Camera _returnvalue)
  (if (not (Variables|Default|GetStatic))
    (Utilities|FlowControl|Sequence
      (:then_0
        (Utilities|Time|SetTimerbyEvent (delegate Custom|FogMovement) 0.1 true))
      (:then_1
        (switch int (Math|Random|RandomIntegerinRange 0 2)
          (:0
            (Class|LocalFogVolumeComponent|SetFogAlbedo (Variables|Default|GetLocalFogVolume) (Utilities|Struct|MakeLinearColor 0.63 0.63 0.63 1.0)))
          (:1
            (Class|LocalFogVolumeComponent|SetFogAlbedo (Variables|Default|GetLocalFogVolume) (Utilities|Struct|MakeLinearColor 0.4 0.4 0.4 1.0))
            (Transformation|AddActorLocalOffset "0.000000,0.000000,-5000.000000" false false))
          (:2
            (Class|LocalFogVolumeComponent|SetFogAlbedo (Variables|Default|GetLocalFogVolume) (Utilities|Struct|MakeLinearColor 0.2 0.2 0.2 1.0))
            (Transformation|AddActorLocalOffset "0.000000,0.000000,-10000.000000" false false))))
      (:then_2
        (EventDispatchers|BindEventtoEDEffects (Variables|Default|GetBP_Camera) (delegate Custom|Effects))))))

(fn ConstructionScript)